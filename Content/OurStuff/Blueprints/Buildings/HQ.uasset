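; HQ building for a turn-based, grid-based hide-and-seek game, where DPS players hold captured Students.
; It moves players between the tile in front of it and its own tile, costing a movement point on entry.
; An entering DPS or Back_Up triggers capture on every held Student, though the Back_Up path reuses the DPS handler.
; A free Student entering releases all captives outside, resets their capture state and reports the count to HideAndSeekGameMode.
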(event Custom|StudentIsEnteringHQ
  (params (Student :type Student%20Object%20Reference))
  (bind _capturedstudents (Variables|Default|GetcapturedStudents))
  ;[0.9669 1 0.1893] Free All Captured Students If A Free Student Enters HQ
  (if (== (Variables|/Game/OurStuff/Blueprints/Grid_Object_Parent.Grid_Object_Parent_C|Getindex Student) (Variables|Default|GetfrontOfDPS))
    (if (not (Variables|/Game/OurStuff/Blueprints/Player/Student.Student_C|GetisCaptured Student))
      (CallFunction|MovePlayerIntoHQ Student)
      (for _array_element _capturedstudents
        (CallFunction|MovePlayerOutOfHQ _array_element)
        (Variables|/Game/OurStuff/Blueprints/Player/HideAndSeekPlayer.HideAndSeekPlayer_C|SetisMovementEnabled _array_element true)
        (Variables|/Game/OurStuff/Blueprints/Player/Student.Student_C|SetisCaptured _array_element false)
        (Variables|/Game/OurStuff/Blueprints/Player/Student.Student_C|SetturnsHasBeenCapturedFor _array_element 0))
      (bind _ashide_and_seek_game_mode (Utilities|Casting|CastToHideAndSeekGameMode (Game|GetGameMode)))
      (Default|StudentsHaveBeenReleased _ashide_and_seek_game_mode (Utilities|Array|Length _capturedstudents))
      (Utilities|Array|Resize (Variables|Default|GetcapturedStudents) 0))))

(event Custom|PlayerIsExitingHQ
  (params (Player :type Hide%20and%20Seek%20Player%20Object%20Reference))
  ;[0 1 0.1634] Decide who is interacting with HQ and how and act appropriately
  (CallFunction|MovePlayerOutOfHQ Player))

(event Custom|MovePlayerIntoHQ
  (params (Player :type Hide%20and%20Seek%20Player%20Object%20Reference))
  ;[1 0.121 0.7169] Handle Moving Players
  (Variables|/Game/OurStuff/Blueprints/Player/HideAndSeekPlayer.HideAndSeekPlayer_C|SetisInHQ Player true)
  (Math|Integer|DecrementInt (Variables|/Game/OurStuff/Blueprints/Player/HideAndSeekPlayer.HideAndSeekPlayer_C|GetmovementPoints Player)
    (:%20%20
      (CallFunction|MovePlayer Player (Variables|Default|Getindex)))))

(event Custom|DPSIsEnteringHQ
  (params (DPS :type Hide%20and%20Seek%20Player%20Object%20Reference))
  ;[1 0.07548 0] Handle DPS entering HQ
  (if (== (Variables|/Game/OurStuff/Blueprints/Grid_Object_Parent.Grid_Object_Parent_C|Getindex DPS) (Variables|Default|GetfrontOfDPS))
    (CallFunction|MovePlayerIntoHQ DPS)
    (for _array_element (Variables|Default|GetcapturedStudents)
      (Default|GetCaptured _array_element))))

(event Custom|MovePlayer
  (params (Player :type Hide%20and%20Seek%20Player%20Object%20Reference) (index :type Integer))
  ;[1 0.121 0.7169] Handle Moving Players
  (Variables|/Game/OurStuff/Blueprints/Grid_Object_Parent.Grid_Object_Parent_C|Setgrid Player (Variables|Default|Getgrid))
  (Default|MovePlayer Player index true))

(event Custom|MovePlayerOutOfHQ
  (params (Player :type Hide%20and%20Seek%20Player%20Object%20Reference))
  ;[1 0.121 0.7169] Handle Moving Players
  (Variables|/Game/OurStuff/Blueprints/Player/HideAndSeekPlayer.HideAndSeekPlayer_C|SetfacingDirection Player (Variables|Default|GetfacingDirectionOnExit))
  (Variables|/Game/OurStuff/Blueprints/Player/HideAndSeekPlayer.HideAndSeekPlayer_C|SetisInHQ Player false)
  (CallFunction|MovePlayer Player (Variables|Default|GetfrontOfDPS)))

(event Custom|PlayerIsEnteringHQ
  (params (Player :type Hide%20and%20Seek%20Player%20Object%20Reference))
  ;[0 1 0.1634] Decide who is interacting with HQ and how and act appropriately
  (bind _asstudent (Utilities|Casting|CastToStudent Player)
    (:then
      (CallFunction|StudentIsEnteringHQ _asstudent))
    (:CastFailed
      (bind _asdps (Utilities|Casting|CastToDPS Player)
        (:then
          (CallFunction|DPSIsEnteringHQ _asdps))
        (:CastFailed
          (bind _asback_up (Utilities|Casting|CastToBack_Up Player))
          (CallFunction|DPSIsEnteringHQ _asback_up))))))

(event EventBeginPlay
  (|CallParentFunction) ; This node is disabled and will not be called.\nDrag off pins to build functionality.
)

(event Collision|EventActorBeginOverlap
  (params (OtherActor :type Actor%20Object%20Reference))
  (|CallParentFunction OtherActor) ; This node is disabled and will not be called.\nDrag off pins to build functionality.
)

(event EventTick
  (params (DeltaSeconds :type Float%20%28single-precision%29))
  (|CallParentFunction DeltaSeconds) ; This node is disabled and will not be called.\nDrag off pins to build functionality.
)

(fn ConstructionScript
  (|CallParentFunction))

(fn AddStudenttoCapturedStudents
  (params (student :type Student%20Object%20Reference))
  (Utilities|Array|Add (Variables|Default|GetcapturedStudents) student)
  (return))

(fn ResetCapturedStudentsSize
  (bind _capturedstudents (Variables|Default|GetcapturedStudents))
  (Utilities|Array|Clear _capturedstudents)
  (Utilities|Array|Resize _capturedstudents 0)
  (return))
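; Flamo is an actor with a minimap point-of-interest marker that removes itself when a DPS turn passes.
; On BeginPlay it sets the marker icon to Bill or Lisa, depending on whether the local player controls Student1 or Student2.
; When notified of the turn change, it removes every widget in the Student or DPS HUD minimap's Delete list, matching the controlled pawn, then destroys itself.
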(event Custom|ClearWidgets
  (bind _returnvalue (Game|GetPlayerController 0))
  (bind _returnvalue_2 (Pawn|GetControlledPawn _returnvalue))
  (bind _asgameplay_pc (Utilities|Casting|CastToGameplayPC _returnvalue))
  (Utilities|Casting|CastToStudent _returnvalue_2
    (:then
      (for _array_element (Variables|/Game/OurStuff/MiniMap/MiniMapWidget.MiniMapWidget_C|GetDelete (Variables|/Game/OurStuff/UI/HUD_Student.HUD_Student_C|GetMiniMapWidget (Variables|/Game/Blueprints/GamePlay/GameplayPC.GameplayPC_C|GetStudentHudRef _asgameplay_pc)))
        (Widget|RemovefromParent _array_element))
      (Actor|DestroyActor))
    (:CastFailed
      (Utilities|Casting|CastToDPS _returnvalue_2)
      (for _array_element_2 (Variables|/Game/OurStuff/MiniMap/MiniMapWidget.MiniMapWidget_C|GetDelete (Variables|/Game/OurStuff/UI/HUD_DPS.HUD_DPS_C|GetMiniMapWidget (Variables|/Game/Blueprints/GamePlay/GameplayPC.GameplayPC_C|GetDPSHudRef _asgameplay_pc)))
        (Widget|RemovefromParent _array_element_2))
      (Actor|DestroyActor))))

(event EventBeginPlay
  (bind _returnvalue (Game|GetPlayerController 0))
  (bind _returnvalue_2 (Pawn|GetControlledPawn _returnvalue))
  (Utilities|Casting|CastToStudent1 _returnvalue_2
    (:then
      (Variables|/Game/OurStuff/MiniMap/PointofInterestComponent.PointofInterestComponent_C|SetIconImage (Variables|Default|GetPointofInterestComponent) "/Game/Textures/Bill.Bill"))
    (:CastFailed
      (Utilities|Casting|CastToStudent2 _returnvalue_2)
      (Variables|/Game/OurStuff/MiniMap/PointofInterestComponent.PointofInterestComponent_C|SetIconImage (Variables|Default|GetPointofInterestComponent) "/Game/Textures/Lisa.Lisa"))))

(event EventNotifyDPSTurnPassed
  (CallFunction|ClearWidgets))

(fn ConstructionScript
  (|CallParentFunction))
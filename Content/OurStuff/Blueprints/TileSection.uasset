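; TileSection is a grid board section that builds its tiles as hierarchical instanced meshes from an X/Y tile count.
; Its construction script stores tile locations and optionally snaps the section to edges of nearby TileSections.
; Objects, objectives and buildings register with it, letting tile queries find occupants by stored index or X/Y bounds.
; Pawn-snapping logic is unwired, as is the building query's not-found return.
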(event EventBeginPlay)

(event EventEndPlay
  (params (EndPlayReason :type EEndPlayReason%20Enum :default "Destroyed"))
  (Utilities|Array|Resize (Variables|Default|GetobjectsWithinGrid) 0)
  (Utilities|Array|Resize (Variables|Default|GetobjectIndices) 0)
  (Utilities|Array|Resize (Variables|Default|GetobjectivesWithinGrid) 0))

(fn ConstructionScript
  (bind _returnvalue (Transformation|GetActorLocation))
  (bind _returnvalue_2 (Transformation|GetActorLocation))
  (bind _returnvalue_3 (Transformation|GetActorLocation))
  (bind _tilesinxdirection (Variables|Default|GettilesInXDirection))
  (bind _tilesinydirection (Variables|Default|GettilesInYDirection))
  (bind _meshfortile (Variables|Default|GetmeshForTile))
  (bind _tilesinxdirection_2 (Variables|Default|GettilesInXDirection))
  (bind _defaultsceneroot (Variables|Default|GetDefaultSceneRoot))
  (bind (_x _y) (Math|Vector|BreakVector _returnvalue))
  (bind (_x_2 _y_2 _z) (Math|Vector|BreakVector _returnvalue_2))
  (bind _returnvalue_4 (StaticMesh|GetBoundingBox _meshfortile))
  (bind _returnvalue_5 (Transformation|GetWorldLocation _defaultsceneroot))
  (bind (_x_3 _y_3) (Math|Vector|BreakVector _returnvalue_3))
  (bind _returnvalue_6 (* _tilesinxdirection _tilesinydirection))
  (bind (_min _max) (Utilities|Struct|BreakBox _returnvalue_4))
  (bind (_x_4 _y_4 _z_2) (Math|Vector|BreakVector _returnvalue_5))
  (bind (_x_5 _y_5 _z_3) (Math|Vector|BreakVector _min))
  (bind (_x_6 _y_6 _z_4) (Math|Vector|BreakVector _max))
  ;[0.08541 1 0.1941 1 24] Create primary mesh through an instanced static mesh
  (bind _returnvalue_7 (AddComponent|AddHierarchicalInstancedStaticMeshComponent false))
  (bind _output_get (Variables|Default|SetTileComponent _returnvalue_7))
  (Components|StaticMesh|SetStaticMesh _output_get _meshfortile)
  (Rendering|Material|SetMaterial _output_get 0 (Variables|Default|GetmeshMaterial))
  (Variables|Default|SetsizeOfMeshX (- _x_6 _x_5))
  (Variables|Default|SetsizeOfMeshY (- _y_6 _y_5))
  (Variables|Default|SetsizeOfMeshZ (- _z_4 _z_3))
  (Variables|Default|SetsizeOfGridX (* (Variables|Default|GettilesInXDirection) (Variables|Default|GetsizeOfMeshX)))
  (Variables|Default|SetsizeOfGridY (* (Variables|Default|GettilesInYDirection) (Variables|Default|GetsizeOfMeshY)))
  ;[0.1083 0.2184 1 1 24] Create an array that holds the location of every mesh
  (Utilities|Array|Resize (Variables|Default|GetlocationsOfMeshes) _returnvalue_6)
  (Variables|Default|SetsizeOfGridArray _returnvalue_6)
  (for _index (range 0 (- _returnvalue_6 1))
    (Utilities|Array|SetArrayElem (Variables|Default|GetlocationsOfMeshes) _index (Math|Vector|MakeVector (* (Math|Integer|%(Integer) _index _tilesinxdirection_2) (Variables|Default|GetsizeOfMeshX)) (* (/ _index _tilesinxdirection_2) (Variables|Default|GetsizeOfMeshY)) 0.0)))
  ;[1 0.2413 0.8033 1 24] Create instances of the mesh
  (for _array_element (Variables|Default|GetlocationsOfMeshes)
    (Components|InstancedStaticMesh|AddInstance (Variables|Default|GetTileComponent) (Math|Conversions|ToTransform(Vector) _array_element))
    ;[0.2015 0.7987 1] Snap this grid to other grids
    (if (Variables|Default|GetsnapThisToOtherGrids)
      (bind _outactors (Actor|GetAllActorsOfClass "TileSection_C"))
      (for _array_element_2 _outactors
        (if (!= _array_element_2 self)
          (LocalVariables|SetpossibleGridToSnapTo _array_element_2)
          (LocalVariables|SetisPastMaxY (>= _y (+ (.Y (Math|Vector|BreakVector (Transformation|GetActorLocation _array_element_2))) (Variables|TileSection_C|GetsizeOfGridY _array_element_2))))
          (LocalVariables|SetisPastMaxX (>= _x (+ (Variables|TileSection_C|GetsizeOfGridX _array_element_2) (.X (Math|Vector|BreakVector (Transformation|GetActorLocation _array_element_2))))))
          (LocalVariables|SetisPastMinY (>= (.Y (Math|Vector|BreakVector (Transformation|GetActorLocation (LocalVariables|GetpossibleGridToSnapTo)))) (+ _y_3 (Variables|Default|GetsizeOfGridY))))
          (LocalVariables|SetisPastMinX (<= (+ _x_3 (Variables|Default|GetsizeOfGridX)) (.X (Math|Vector|BreakVector (Transformation|GetActorLocation (LocalVariables|GetpossibleGridToSnapTo))))))
          (LocalVariables|SetisWithinRangeOfMaxY (and (>= _y (+ (.Y (Math|Vector|BreakVector (Transformation|GetActorLocation _array_element_2))) (Variables|TileSection_C|GetsizeOfGridY _array_element_2))) (<= _y (+ (+ (.Y (Math|Vector|BreakVector (Transformation|GetActorLocation _array_element_2))) (Variables|TileSection_C|GetsizeOfGridY _array_element_2)) (* (Variables|Default|GetsizeOfMeshY) (Variables|Default|GetrangeForGridSnap))))))
          (LocalVariables|SetisWithinRangeOfMaxX (and (>= _x (+ (Variables|TileSection_C|GetsizeOfGridX _array_element_2) (.X (Math|Vector|BreakVector (Transformation|GetActorLocation _array_element_2))))) (<= (- (Math|Float|Absolute(Float) _x) (+ (Variables|TileSection_C|GetsizeOfGridX _array_element_2) (.X (Math|Vector|BreakVector (Transformation|GetActorLocation _array_element_2))))) (* (Variables|Default|GetrangeForGridSnap) (Variables|Default|GetsizeOfMeshX)))))
          (LocalVariables|SetisWithinRangeOfMinX (and (>= (- (+ _x_3 (Variables|Default|GetsizeOfGridX)) (Variables|Default|GetsizeOfMeshX)) (- (.X (Math|Vector|BreakVector (Transformation|GetActorLocation (LocalVariables|GetpossibleGridToSnapTo)))) (* (Variables|Default|GetrangeForGridSnap) (Variables|Default|GetsizeOfMeshX)))) (<= (- (+ _x_3 (Variables|Default|GetsizeOfGridX)) (Variables|Default|GetsizeOfMeshX)) (- (.X (Math|Vector|BreakVector (Transformation|GetActorLocation (LocalVariables|GetpossibleGridToSnapTo)))) (/ (Variables|Default|GetsizeOfMeshX) 2.0)))))
          (LocalVariables|SetisWithinRangeOfMinY (and (<= (- (+ _y_3 (Variables|Default|GetsizeOfGridY)) (Variables|Default|GetsizeOfMeshY)) (- (.Y (Math|Vector|BreakVector (Transformation|GetActorLocation (LocalVariables|GetpossibleGridToSnapTo)))) (/ (Variables|Default|GetsizeOfMeshY) 2.0))) (>= (- (+ _y_3 (Variables|Default|GetsizeOfGridY)) (Variables|Default|GetsizeOfMeshY)) (- (.Y (Math|Vector|BreakVector (Transformation|GetActorLocation (LocalVariables|GetpossibleGridToSnapTo)))) (* (Variables|Default|GetsizeOfMeshY) (Variables|Default|GetrangeForGridSnap))))))
          (if (Math|Boolean|ANDBoolean (LocalVariables|GetisWithinRangeOfMaxX) (not (LocalVariables|GetisPastMaxY)) (not (LocalVariables|GetisPastMinY)) (Variables|Default|GetsnapOnPositiveX))
            (Transformation|SetWorldLocation (Variables|Default|GetDefaultSceneRoot) (Math|Vector|MakeVector (- _x_2 (.X (Math|Vector|BreakVector (- _returnvalue_2 (+ (Transformation|GetActorLocation (LocalVariables|GetpossibleGridToSnapTo)) (Math|Vector|MakeVector (Variables|TileSection_C|GetsizeOfGridX (LocalVariables|GetpossibleGridToSnapTo)) 0.0 0.0)))))) (- _y_2 (Math|Float|%(Float) (.Y (Math|Vector|BreakVector (- _returnvalue_2 (+ (Transformation|GetActorLocation (LocalVariables|GetpossibleGridToSnapTo)) (Math|Vector|MakeVector (Variables|TileSection_C|GetsizeOfGridX (LocalVariables|GetpossibleGridToSnapTo)) 0.0 0.0))))) (Variables|Default|GetsizeOfMeshY))) (- _z (.Z (Math|Vector|BreakVector (- _returnvalue_2 (+ (Transformation|GetActorLocation (LocalVariables|GetpossibleGridToSnapTo)) (Math|Vector|MakeVector (Variables|TileSection_C|GetsizeOfGridX (LocalVariables|GetpossibleGridToSnapTo)) 0.0 0.0))))))) false false)
            (Transformation|SetActorLocation (Math|Vector|MakeVector (- _x_2 (.X (Math|Vector|BreakVector (- _returnvalue_2 (+ (Transformation|GetActorLocation (LocalVariables|GetpossibleGridToSnapTo)) (Math|Vector|MakeVector (Variables|TileSection_C|GetsizeOfGridX (LocalVariables|GetpossibleGridToSnapTo)) 0.0 0.0)))))) (- _y_2 (Math|Float|%(Float) (.Y (Math|Vector|BreakVector (- _returnvalue_2 (+ (Transformation|GetActorLocation (LocalVariables|GetpossibleGridToSnapTo)) (Math|Vector|MakeVector (Variables|TileSection_C|GetsizeOfGridX (LocalVariables|GetpossibleGridToSnapTo)) 0.0 0.0))))) (Variables|Default|GetsizeOfMeshY))) (- _z (.Z (Math|Vector|BreakVector (- _returnvalue_2 (+ (Transformation|GetActorLocation (LocalVariables|GetpossibleGridToSnapTo)) (Math|Vector|MakeVector (Variables|TileSection_C|GetsizeOfGridX (LocalVariables|GetpossibleGridToSnapTo)) 0.0 0.0))))))) false false)
            (else
              (if (Math|Boolean|ANDBoolean (LocalVariables|GetisWithinRangeOfMaxY) (not (LocalVariables|GetisPastMaxX)) (not (LocalVariables|GetisPastMinX)) (Variables|Default|GetsnapOnPositiveY))
                (Transformation|SetWorldLocation (Variables|Default|GetDefaultSceneRoot) (Math|Vector|MakeVector (- _x_4 (Math|Float|%(Float) (.X (Math|Vector|BreakVector (- _returnvalue_5 (+ (Transformation|GetWorldLocation (Variables|TileSection_C|GetDefaultSceneRoot (LocalVariables|GetpossibleGridToSnapTo))) (Math|Vector|MakeVector 0.0 (Variables|TileSection_C|GetsizeOfGridY (LocalVariables|GetpossibleGridToSnapTo)) 0.0))))) (Variables|Default|GetsizeOfMeshX))) (- _y_4 (.Y (Math|Vector|BreakVector (- _returnvalue_5 (+ (Transformation|GetWorldLocation (Variables|TileSection_C|GetDefaultSceneRoot (LocalVariables|GetpossibleGridToSnapTo))) (Math|Vector|MakeVector 0.0 (Variables|TileSection_C|GetsizeOfGridY (LocalVariables|GetpossibleGridToSnapTo)) 0.0)))))) (- _z_2 (.Z (Math|Vector|BreakVector (- _returnvalue_5 (+ (Transformation|GetWorldLocation (Variables|TileSection_C|GetDefaultSceneRoot (LocalVariables|GetpossibleGridToSnapTo))) (Math|Vector|MakeVector 0.0 (Variables|TileSection_C|GetsizeOfGridY (LocalVariables|GetpossibleGridToSnapTo)) 0.0))))))) false false)
                (Transformation|SetActorLocation (Math|Vector|MakeVector (- _x_4 (Math|Float|%(Float) (.X (Math|Vector|BreakVector (- _returnvalue_5 (+ (Transformation|GetWorldLocation (Variables|TileSection_C|GetDefaultSceneRoot (LocalVariables|GetpossibleGridToSnapTo))) (Math|Vector|MakeVector 0.0 (Variables|TileSection_C|GetsizeOfGridY (LocalVariables|GetpossibleGridToSnapTo)) 0.0))))) (Variables|Default|GetsizeOfMeshX))) (- _y_4 (.Y (Math|Vector|BreakVector (- _returnvalue_5 (+ (Transformation|GetWorldLocation (Variables|TileSection_C|GetDefaultSceneRoot (LocalVariables|GetpossibleGridToSnapTo))) (Math|Vector|MakeVector 0.0 (Variables|TileSection_C|GetsizeOfGridY (LocalVariables|GetpossibleGridToSnapTo)) 0.0)))))) (- _z_2 (.Z (Math|Vector|BreakVector (- _returnvalue_5 (+ (Transformation|GetWorldLocation (Variables|TileSection_C|GetDefaultSceneRoot (LocalVariables|GetpossibleGridToSnapTo))) (Math|Vector|MakeVector 0.0 (Variables|TileSection_C|GetsizeOfGridY (LocalVariables|GetpossibleGridToSnapTo)) 0.0))))))) false false))
              (if (Math|Boolean|ANDBoolean (LocalVariables|GetisWithinRangeOfMinY) (not (LocalVariables|GetisPastMinX)) (not (LocalVariables|GetisPastMaxX)) (Variables|Default|GetsnapOnNegativeY))
                (Transformation|SetWorldLocation (Variables|Default|GetDefaultSceneRoot) (Math|Vector|MakeVector (- (.X (Math|Vector|BreakVector (+ (Math|Vector|MakeVector 0.0 (- (Variables|Default|GetsizeOfGridY) (/ (Variables|Default|GetsizeOfMeshY) 2.0)) 0.0) (Transformation|GetWorldLocation (Variables|Default|GetDefaultSceneRoot))))) (Math|Float|%(Float) (.X (Math|Vector|BreakVector (- (+ (Math|Vector|MakeVector 0.0 (- (Variables|Default|GetsizeOfGridY) (/ (Variables|Default|GetsizeOfMeshY) 2.0)) 0.0) (Transformation|GetWorldLocation (Variables|Default|GetDefaultSceneRoot))) (Transformation|GetWorldLocation (Variables|TileSection_C|GetDefaultSceneRoot (LocalVariables|GetpossibleGridToSnapTo)))))) (Variables|Default|GetsizeOfMeshX))) (- (- (.Y (Math|Vector|BreakVector (+ (Math|Vector|MakeVector 0.0 (- (Variables|Default|GetsizeOfGridY) (/ (Variables|Default|GetsizeOfMeshY) 2.0)) 0.0) (Transformation|GetWorldLocation (Variables|Default|GetDefaultSceneRoot))))) (.Y (Math|Vector|BreakVector (- (+ (Math|Vector|MakeVector 0.0 (- (Variables|Default|GetsizeOfGridY) (/ (Variables|Default|GetsizeOfMeshY) 2.0)) 0.0) (Transformation|GetWorldLocation (Variables|Default|GetDefaultSceneRoot))) (Transformation|GetWorldLocation (Variables|TileSection_C|GetDefaultSceneRoot (LocalVariables|GetpossibleGridToSnapTo))))))) (Variables|Default|GetsizeOfGridY)) (- (.Z (Math|Vector|BreakVector (+ (Math|Vector|MakeVector 0.0 (- (Variables|Default|GetsizeOfGridY) (/ (Variables|Default|GetsizeOfMeshY) 2.0)) 0.0) (Transformation|GetWorldLocation (Variables|Default|GetDefaultSceneRoot))))) (.Z (Math|Vector|BreakVector (- (+ (Math|Vector|MakeVector 0.0 (- (Variables|Default|GetsizeOfGridY) (/ (Variables|Default|GetsizeOfMeshY) 2.0)) 0.0) (Transformation|GetWorldLocation (Variables|Default|GetDefaultSceneRoot))) (Transformation|GetWorldLocation (Variables|TileSection_C|GetDefaultSceneRoot (LocalVariables|GetpossibleGridToSnapTo)))))))) false false)
                (Transformation|SetActorLocation (Math|Vector|MakeVector (- (.X (Math|Vector|BreakVector (+ (Math|Vector|MakeVector 0.0 (- (Variables|Default|GetsizeOfGridY) (/ (Variables|Default|GetsizeOfMeshY) 2.0)) 0.0) (Transformation|GetWorldLocation (Variables|Default|GetDefaultSceneRoot))))) (Math|Float|%(Float) (.X (Math|Vector|BreakVector (- (+ (Math|Vector|MakeVector 0.0 (- (Variables|Default|GetsizeOfGridY) (/ (Variables|Default|GetsizeOfMeshY) 2.0)) 0.0) (Transformation|GetWorldLocation (Variables|Default|GetDefaultSceneRoot))) (Transformation|GetWorldLocation (Variables|TileSection_C|GetDefaultSceneRoot (LocalVariables|GetpossibleGridToSnapTo)))))) (Variables|Default|GetsizeOfMeshX))) (- (- (.Y (Math|Vector|BreakVector (+ (Math|Vector|MakeVector 0.0 (- (Variables|Default|GetsizeOfGridY) (/ (Variables|Default|GetsizeOfMeshY) 2.0)) 0.0) (Transformation|GetWorldLocation (Variables|Default|GetDefaultSceneRoot))))) (.Y (Math|Vector|BreakVector (- (+ (Math|Vector|MakeVector 0.0 (- (Variables|Default|GetsizeOfGridY) (/ (Variables|Default|GetsizeOfMeshY) 2.0)) 0.0) (Transformation|GetWorldLocation (Variables|Default|GetDefaultSceneRoot))) (Transformation|GetWorldLocation (Variables|TileSection_C|GetDefaultSceneRoot (LocalVariables|GetpossibleGridToSnapTo))))))) (Variables|Default|GetsizeOfGridY)) (- (.Z (Math|Vector|BreakVector (+ (Math|Vector|MakeVector 0.0 (- (Variables|Default|GetsizeOfGridY) (/ (Variables|Default|GetsizeOfMeshY) 2.0)) 0.0) (Transformation|GetWorldLocation (Variables|Default|GetDefaultSceneRoot))))) (.Z (Math|Vector|BreakVector (- (+ (Math|Vector|MakeVector 0.0 (- (Variables|Default|GetsizeOfGridY) (/ (Variables|Default|GetsizeOfMeshY) 2.0)) 0.0) (Transformation|GetWorldLocation (Variables|Default|GetDefaultSceneRoot))) (Transformation|GetWorldLocation (Variables|TileSection_C|GetDefaultSceneRoot (LocalVariables|GetpossibleGridToSnapTo)))))))) false false))
              (if (Math|Boolean|ANDBoolean (LocalVariables|GetisWithinRangeOfMinX) (not (LocalVariables|GetisPastMaxY)) (not (LocalVariables|GetisPastMinY)) (Variables|Default|GetsnapOnNegativeX))
                (Transformation|SetWorldLocation (Variables|Default|GetDefaultSceneRoot) (Math|Vector|MakeVector (- (- (.X (Math|Vector|BreakVector (+ (Math|Vector|MakeVector (- (Variables|Default|GetsizeOfGridX) (/ (Variables|Default|GetsizeOfMeshX) 2.0)) 0.0 0.0) (Transformation|GetWorldLocation (Variables|Default|GetDefaultSceneRoot))))) (.X (Math|Vector|BreakVector (- (+ (Math|Vector|MakeVector (- (Variables|Default|GetsizeOfGridX) (/ (Variables|Default|GetsizeOfMeshX) 2.0)) 0.0 0.0) (Transformation|GetWorldLocation (Variables|Default|GetDefaultSceneRoot))) (Transformation|GetWorldLocation (Variables|TileSection_C|GetDefaultSceneRoot (LocalVariables|GetpossibleGridToSnapTo))))))) (Variables|Default|GetsizeOfGridX)) (- (.Y (Math|Vector|BreakVector (+ (Math|Vector|MakeVector (- (Variables|Default|GetsizeOfGridX) (/ (Variables|Default|GetsizeOfMeshX) 2.0)) 0.0 0.0) (Transformation|GetWorldLocation (Variables|Default|GetDefaultSceneRoot))))) (Math|Float|%(Float) (.Y (Math|Vector|BreakVector (- (+ (Math|Vector|MakeVector (- (Variables|Default|GetsizeOfGridX) (/ (Variables|Default|GetsizeOfMeshX) 2.0)) 0.0 0.0) (Transformation|GetWorldLocation (Variables|Default|GetDefaultSceneRoot))) (Transformation|GetWorldLocation (Variables|TileSection_C|GetDefaultSceneRoot (LocalVariables|GetpossibleGridToSnapTo)))))) (Variables|Default|GetsizeOfMeshX))) (- (.Z (Math|Vector|BreakVector (+ (Math|Vector|MakeVector (- (Variables|Default|GetsizeOfGridX) (/ (Variables|Default|GetsizeOfMeshX) 2.0)) 0.0 0.0) (Transformation|GetWorldLocation (Variables|Default|GetDefaultSceneRoot))))) (.Z (Math|Vector|BreakVector (- (+ (Math|Vector|MakeVector (- (Variables|Default|GetsizeOfGridX) (/ (Variables|Default|GetsizeOfMeshX) 2.0)) 0.0 0.0) (Transformation|GetWorldLocation (Variables|Default|GetDefaultSceneRoot))) (Transformation|GetWorldLocation (Variables|TileSection_C|GetDefaultSceneRoot (LocalVariables|GetpossibleGridToSnapTo)))))))) false false)
                (Transformation|SetActorLocation (Math|Vector|MakeVector (- (- (.X (Math|Vector|BreakVector (+ (Math|Vector|MakeVector (- (Variables|Default|GetsizeOfGridX) (/ (Variables|Default|GetsizeOfMeshX) 2.0)) 0.0 0.0) (Transformation|GetWorldLocation (Variables|Default|GetDefaultSceneRoot))))) (.X (Math|Vector|BreakVector (- (+ (Math|Vector|MakeVector (- (Variables|Default|GetsizeOfGridX) (/ (Variables|Default|GetsizeOfMeshX) 2.0)) 0.0 0.0) (Transformation|GetWorldLocation (Variables|Default|GetDefaultSceneRoot))) (Transformation|GetWorldLocation (Variables|TileSection_C|GetDefaultSceneRoot (LocalVariables|GetpossibleGridToSnapTo))))))) (Variables|Default|GetsizeOfGridX)) (- (.Y (Math|Vector|BreakVector (+ (Math|Vector|MakeVector (- (Variables|Default|GetsizeOfGridX) (/ (Variables|Default|GetsizeOfMeshX) 2.0)) 0.0 0.0) (Transformation|GetWorldLocation (Variables|Default|GetDefaultSceneRoot))))) (Math|Float|%(Float) (.Y (Math|Vector|BreakVector (- (+ (Math|Vector|MakeVector (- (Variables|Default|GetsizeOfGridX) (/ (Variables|Default|GetsizeOfMeshX) 2.0)) 0.0 0.0) (Transformation|GetWorldLocation (Variables|Default|GetDefaultSceneRoot))) (Transformation|GetWorldLocation (Variables|TileSection_C|GetDefaultSceneRoot (LocalVariables|GetpossibleGridToSnapTo)))))) (Variables|Default|GetsizeOfMeshX))) (- (.Z (Math|Vector|BreakVector (+ (Math|Vector|MakeVector (- (Variables|Default|GetsizeOfGridX) (/ (Variables|Default|GetsizeOfMeshX) 2.0)) 0.0 0.0) (Transformation|GetWorldLocation (Variables|Default|GetDefaultSceneRoot))))) (.Z (Math|Vector|BreakVector (- (+ (Math|Vector|MakeVector (- (Variables|Default|GetsizeOfGridX) (/ (Variables|Default|GetsizeOfMeshX) 2.0)) 0.0 0.0) (Transformation|GetWorldLocation (Variables|Default|GetDefaultSceneRoot))) (Transformation|GetWorldLocation (Variables|TileSection_C|GetDefaultSceneRoot (LocalVariables|GetpossibleGridToSnapTo)))))))) false false)))))))))

(fn SnapPawnstoGrid)

(fn CalculateDistancefromTile
  (params (Location :type Float%20%28single-precision%29) (DirectionSize :type Float%20%28single-precision%29))
  (return (+ (- Location (Math|Float|%(Float) Location DirectionSize)) (/ DirectionSize 2.0))))

(fn CenterPawnActors)

(fn GetCenterOfClosestTile
  (params (WorldLocation :type Vector))
  (bind (_x _y _z) (Math|Vector|BreakVector WorldLocation))
  (bind _centeroftile (CallFunction|CalculateDistancefromTile _x (Variables|Default|GetsizeOfMeshX)))
  (bind _centeroftile_2 (CallFunction|CalculateDistancefromTile _y (Variables|Default|GetsizeOfMeshY)))
  (return (Math|Vector|MakeVector _centeroftile _centeroftile_2 _z)))

(fn GetTileLocationfromIndex
  (params (Index :type Integer))
  (return (+ (Utilities|Array|Get(acopy) (Variables|Default|GetlocationsOfMeshes) Index) (Transformation|GetActorLocation))))

(fn RegisterObject
  (params (object :type Grid%20Object%20Parent%20Object%20Reference))
  (Utilities|Array|Add (Variables|Default|GetobjectsWithinGrid) object)
  (Utilities|Array|Add (Variables|Default|GetobjectIndices) (Variables|/Game/OurStuff/Blueprints/Grid_Object_Parent.Grid_Object_Parent_C|Getindex object)))

(fn RegisterObjective
  (params (objective :type Objective%20Object%20Reference))
  (Utilities|Array|Add (Variables|Default|GetobjectivesWithinGrid) objective))

(fn CheckifIndexIsinAnObjective
  (params (index :type Integer))
  (for _array_element (Variables|Default|GetobjectivesWithinGrid)
    ;[0.05069 1 0] Check if the index is within the x-bounds of the objective
    (bind _worldlocation (CallFunction|GetTileLocationfromIndex index))
    (bind _output_get (LocalVariables|SetisWithinXBounds (and (<= (.X (Math|Vector|BreakVector _worldlocation)) (.X (Math|Vector|BreakVector (+ (.Origin (Collision|GetComponentBounds (Variables|/Game/OurStuff/Blueprints/Objective.Objective_C|GetObjectiveBounds _array_element))) (Math|Vector|MakeVector (.X (Math|Vector|BreakVector (.BoxExtent (Collision|GetComponentBounds (Variables|/Game/OurStuff/Blueprints/Objective.Objective_C|GetObjectiveBounds _array_element))))) 0.0 0.0))))) (>= (.X (Math|Vector|BreakVector _worldlocation)) (.X (Math|Vector|BreakVector (- (.Origin (Collision|GetComponentBounds (Variables|/Game/OurStuff/Blueprints/Objective.Objective_C|GetObjectiveBounds _array_element))) (Math|Vector|MakeVector (.X (Math|Vector|BreakVector (.BoxExtent (Collision|GetComponentBounds (Variables|/Game/OurStuff/Blueprints/Objective.Objective_C|GetObjectiveBounds _array_element))))) 0.0 0.0))))))))
    (if _output_get
      ;[1 0.2567 0] Check if the index is within the y-bounds of the objective
      (bind _worldlocation_2 (CallFunction|GetTileLocationfromIndex index))
      (bind _output_get_2 (LocalVariables|SetisWithinYBounds (and (<= (.Y (Math|Vector|BreakVector _worldlocation_2)) (.Y (Math|Vector|BreakVector (+ (.Origin (Collision|GetComponentBounds (Variables|/Game/OurStuff/Blueprints/Objective.Objective_C|GetObjectiveBounds _array_element))) (Math|Vector|MakeVector 0.0 (.Y (Math|Vector|BreakVector (.BoxExtent (Collision|GetComponentBounds (Variables|/Game/OurStuff/Blueprints/Objective.Objective_C|GetObjectiveBounds _array_element))))) 0.0))))) (>= (.Y (Math|Vector|BreakVector _worldlocation_2)) (.Y (Math|Vector|BreakVector (- (.Origin (Collision|GetComponentBounds (Variables|/Game/OurStuff/Blueprints/Objective.Objective_C|GetObjectiveBounds _array_element))) (Math|Vector|MakeVector 0.0 (.Y (Math|Vector|BreakVector (.BoxExtent (Collision|GetComponentBounds (Variables|/Game/OurStuff/Blueprints/Objective.Objective_C|GetObjectiveBounds _array_element))))) 0.0))))))))
      (if _output_get_2
        (return true _array_element))))
  (return false (LocalVariables|GetNULL_OBJECTIVE)))

(fn CheckifIndexIsTakenbyAnObject
  (params (index :type Integer))
  (for (_array_element _array_index) (Variables|Default|GetobjectIndices)
    (if (== _array_element index)
      (return true (Utilities|Array|Get(acopy) (Variables|Default|GetobjectsWithinGrid) _array_index))))
  (return false (LocalVariables|GetNULL_OBJECT)))

(fn CheckifIndexIsTakenbyBuilding
  (params (index :type Integer))
  (for _array_element (Variables|Default|GetbuildingsWithinGrid)
    ;[0.05069 1 0] Check if the index is within the x-bounds of the objective
    (bind _worldlocation (CallFunction|GetTileLocationfromIndex index))
    (bind _output_get (LocalVariables|SetisWithinRangeOfX (and (<= (.X (Math|Vector|BreakVector _worldlocation)) (.X (Math|Vector|BreakVector (+ (.Origin (Collision|GetComponentBounds (Variables|/Game/OurStuff/Blueprints/Buildings/Building.Building_C|GetBuildingBounds _array_element))) (Math|Vector|MakeVector (.X (Math|Vector|BreakVector (.BoxExtent (Collision|GetComponentBounds (Variables|/Game/OurStuff/Blueprints/Buildings/Building.Building_C|GetBuildingBounds _array_element))))) 0.0 0.0))))) (>= (.X (Math|Vector|BreakVector _worldlocation)) (.X (Math|Vector|BreakVector (- (.Origin (Collision|GetComponentBounds (Variables|/Game/OurStuff/Blueprints/Buildings/Building.Building_C|GetBuildingBounds _array_element))) (Math|Vector|MakeVector (.X (Math|Vector|BreakVector (.BoxExtent (Collision|GetComponentBounds (Variables|/Game/OurStuff/Blueprints/Buildings/Building.Building_C|GetBuildingBounds _array_element))))) 0.0 0.0))))))))
    (if _output_get
      ;[1 0.2567 0] Check if the index is within the y-bounds of the objective
      (bind _worldlocation_2 (CallFunction|GetTileLocationfromIndex index))
      (bind _output_get_2 (LocalVariables|SetisWithinRangeOfY (and (<= (.Y (Math|Vector|BreakVector _worldlocation_2)) (.Y (Math|Vector|BreakVector (+ (.Origin (Collision|GetComponentBounds (Variables|/Game/OurStuff/Blueprints/Buildings/Building.Building_C|GetBuildingBounds _array_element))) (Math|Vector|MakeVector 0.0 (.Y (Math|Vector|BreakVector (.BoxExtent (Collision|GetComponentBounds (Variables|/Game/OurStuff/Blueprints/Buildings/Building.Building_C|GetBuildingBounds _array_element))))) 0.0))))) (>= (.Y (Math|Vector|BreakVector _worldlocation_2)) (.Y (Math|Vector|BreakVector (- (.Origin (Collision|GetComponentBounds (Variables|/Game/OurStuff/Blueprints/Buildings/Building.Building_C|GetBuildingBounds _array_element))) (Math|Vector|MakeVector 0.0 (.Y (Math|Vector|BreakVector (.BoxExtent (Collision|GetComponentBounds (Variables|/Game/OurStuff/Blueprints/Buildings/Building.Building_C|GetBuildingBounds _array_element))))) 0.0))))))))
      (if _output_get_2
        (return true _array_element)))))

(fn RegisterBuilding
  (params (building :type Building%20Object%20Reference))
  (Utilities|Array|Add (Variables|Default|GetbuildingsWithinGrid) building))
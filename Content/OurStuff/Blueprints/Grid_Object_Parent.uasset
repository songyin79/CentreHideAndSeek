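; Base actor for objects that sit on TileSection grids, registering itself with its grid at BeginPlay.
; With SnapToGrid on, the construction script keeps or searches for the grid whose bounds contain the actor, falling back to the first TileSection found.
; It converts the half-tile-offset location to a flattened tile index, then moves GridAnchor to that tile with a height offset.
; A separate index conversion for movement skips the per-axis tile flooring.
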(event EventBeginPlay
  (Default|RegisterObject (Variables|Default|Getgrid) self))

(fn ConstructionScript
  (bind _returnvalue (Transformation|GetActorLocation))
  (bind _returnvalue_2 (Transformation|GetActorLocation))
  (bind (_x _y _z) (Math|Vector|BreakVector _returnvalue))
  (if (Variables|Default|GetsnapToGrid)
    ;[1 0.2478 0] Find the Correct Grid
    (bind _iswithingrid (CallFunction|IsWithinRangeOfGrid _returnvalue_2 (Variables|Default|Getgrid)))
    (if _iswithingrid
      _
      (else
        (bind _grid (CallFunction|FindGridCorrelatingtoAWorldLocation _returnvalue_2))
        (Variables|Default|Setgrid _grid)))
    ;[1 0.02672 0.7989] Snap the object to the grid
    (bind _index (CallFunction|ConvertWorldLocationtoIndex (Math|Vector|MakeVector (+ (/ (Variables|/Game/OurStuff/Blueprints/TileSection.TileSection_C|GetsizeOfMeshX (Variables|Default|Getgrid)) 2.0) _x) (+ _y (/ (Variables|/Game/OurStuff/Blueprints/TileSection.TileSection_C|GetsizeOfMeshY (Variables|Default|Getgrid)) 2.0)) _z) false))
    (Variables|Default|Setindex _index)
    (if (Variables|Default|GetsnapToGrid)
      (bind _worldlocation (Default|GetTileLocationfromIndex (Variables|Default|Getgrid) (Variables|Default|Getindex)))
      (Transformation|SetWorldLocation (Variables|Default|GetGridAnchor) (+ _worldlocation (Math|Vector|MakeVector 0.0 0.0 (+ (.Z (Math|Vector|BreakVector (Variables|Default|GetSizeOfMesh))) (Variables|/Game/OurStuff/Blueprints/TileSection.TileSection_C|GetsizeOfMeshZ (Variables|Default|Getgrid)) (- (.Z (Math|Vector|BreakVector (Transformation|GetWorldLocation (Variables|Default|GetGridAnchor)))) (.Z (Math|Vector|BreakVector (Transformation|GetWorldLocation (Variables|/Game/OurStuff/Blueprints/TileSection.TileSection_C|GetDefaultSceneRoot (Variables|Default|Getgrid))))))))) false false))))

(fn ConvertWorldLocationtoIndex
  (params (worldLocation :type Vector) (shouldNotCalculateIndex :type Boolean))
  (bind _grid (Variables|Default|Getgrid))
  (bind _grid_2 (Variables|Default|Getgrid))
  (bind _returnvalue (Transformation|GetActorLocation _grid))
  (bind _sizeofmeshy (Variables|/Game/OurStuff/Blueprints/TileSection.TileSection_C|GetsizeOfMeshY _grid_2))
  (bind _sizeofmeshx (Variables|/Game/OurStuff/Blueprints/TileSection.TileSection_C|GetsizeOfMeshX _grid_2))
  (bind _returnvalue_2 (- worldLocation _returnvalue))
  (bind (_x _y) (Math|Vector|BreakVector _returnvalue_2))
  (return (Math|Float|Round (+ (/ (- _x (Math|Float|%(Float) _x _sizeofmeshx)) _sizeofmeshx) (* (Variables|/Game/OurStuff/Blueprints/TileSection.TileSection_C|GettilesInXDirection _grid_2) (/ (- _y (Math|Float|%(Float) _y _sizeofmeshy)) _sizeofmeshy))))))

(fn IsWithinRangeOfGrid
  (params (worldLocation :type Vector) (grid :type Tile%20Section%20Object%20Reference))
  (bind _returnvalue (Transformation|GetActorLocation grid))
  (bind (_x _y) (Math|Vector|BreakVector worldLocation))
  (bind _sizeofmeshx (Variables|/Game/OurStuff/Blueprints/TileSection.TileSection_C|GetsizeOfMeshX grid))
  (bind _sizeofmeshy (Variables|/Game/OurStuff/Blueprints/TileSection.TileSection_C|GetsizeOfMeshY grid))
  (bind (_x_2 _y_2) (Math|Vector|BreakVector _returnvalue))
  (bind _returnvalue_2 (/ _sizeofmeshy 2.0))
  (bind _returnvalue_3 (/ _sizeofmeshx 2.0))
  (if (Utilities|IsValid grid)
    (return (Math|Boolean|ANDBoolean (<= _x (- (+ _x_2 (Variables|/Game/OurStuff/Blueprints/TileSection.TileSection_C|GetsizeOfGridX grid)) _returnvalue_3)) (<= _y (- (+ _y_2 (Variables|/Game/OurStuff/Blueprints/TileSection.TileSection_C|GetsizeOfGridY grid)) _returnvalue_2)) (>= _x (- _x_2 _returnvalue_3)) (>= _y (- _y_2 _returnvalue_2))))
    (else
      (return false))))

(fn FindGridCorrelatingtoAWorldLocation
  (params (worldLocation :type Vector))
  (LocalVariables|SetfoundGrid false)
  (bind _outactors (Actor|GetAllActorsOfClass "/Game/OurStuff/Blueprints/TileSection.TileSection_C"))
  (LocalVariables|SetreturnGrid (Utilities|Array|Get(acopy) _outactors))
  (bind _array_element (Utilities|Array|ForEachLoopwithBreak _outactors :!label _label)
    (:LoopBody
      (bind _iswithingrid (CallFunction|IsWithinRangeOfGrid worldLocation _array_element))
      (if _iswithingrid
        (LocalVariables|SetreturnGrid _array_element)
        (LocalVariables|SetfoundGrid true)
        (goto _label Break)))
    (:Completed
      (return (LocalVariables|GetreturnGrid) (LocalVariables|GetfoundGrid)))))

(fn ConvertWorldLocationtoIndexforMovement
  (params (worldLocation :type Vector))
  (bind _grid (Variables|Default|Getgrid))
  (bind _grid_2 (Variables|Default|Getgrid))
  (bind _returnvalue (Transformation|GetActorLocation _grid))
  (bind _returnvalue_2 (- worldLocation _returnvalue))
  (bind (_x _y) (Math|Vector|BreakVector _returnvalue_2))
  (return (Math|Float|Round (+ (/ _x (Variables|/Game/OurStuff/Blueprints/TileSection.TileSection_C|GetsizeOfMeshX _grid_2)) (* (Variables|/Game/OurStuff/Blueprints/TileSection.TileSection_C|GettilesInXDirection _grid_2) (/ _y (Variables|/Game/OurStuff/Blueprints/TileSection.TileSection_C|GetsizeOfMeshY _grid_2)))))))
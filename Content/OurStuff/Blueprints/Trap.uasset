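; Trap actor that catches Student pawns, staying hidden when the local player controls a Student and visible otherwise.
; A Student overlap reveals the trap and particles, flags the victim as trapped and turns off its mesh's owner-only visibility.
; It also spawns a Whistle2 point-of-interest marker, with an icon chosen by the victim's class.
; When notified that the DPS turn passed, it restores the victim's owner-only visibility and destroys itself if used.
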(event OnComponentBeginOverlap(Box)
  (params (OverlappedComponent :type Primitive%20Component%20Object%20Reference) (OtherActor :type Actor%20Object%20Reference) (OtherComp :type Primitive%20Component%20Object%20Reference) (OtherBodyIndex :type Integer) (bFromSweep :type Boolean) (SweepResult :type Hit%20Result%20Structure%20%28by%20ref%29))
  (Utilities|Casting|CastToStudent OtherActor)
  (Rendering|SetVisibility (Variables|Default|GetStaticMesh) true true)
  (CallFunction|Overlapped OtherActor)
  (Utilities|Casting|CastToStudent1 OtherActor
    (:then
      (Variables|/Game/OurStuff/MiniMap/PointofInterestComponent.PointofInterestComponent_C|SetIconImage (Variables|/Game/OurStuff/Blueprints/Whistle2.Whistle2_C|GetPointofInterestComponent (stale Custom|Overlapped _returnvalue)) "/Game/Textures/Bill.Bill"))
    (:CastFailed
      (Utilities|Casting|CastToDPS2 OtherActor)
      (Variables|/Game/OurStuff/MiniMap/PointofInterestComponent.PointofInterestComponent_C|SetIconImage (Variables|/Game/OurStuff/Blueprints/Whistle2.Whistle2_C|GetPointofInterestComponent (stale Custom|Overlapped _returnvalue)) "/Game/Textures/Lisa.Lisa"))))

(event Custom|Overlapped
  (params (Actor :type Actor%20Object%20Reference))
  (bind (_asstudent _bsuccess) (Utilities|Casting|CastToStudent Actor))
  (bind _playermesh (Variables|/Game/OurStuff/Blueprints/Player/HideAndSeekPlayer.HideAndSeekPlayer_C|GetPlayerMesh _asstudent))
  (if _bsuccess
    (Variables|/Game/OurStuff/Blueprints/Player/Student.Student_C|SetisTrapped _asstudent true)
    (Rendering|SetOnlyOwnerSee _playermesh false :!class /Script/Engine.PrimitiveComponent)
    (Variables|Default|SetTrappedKid _playermesh)
    (bind _asgrid_object_parent (Utilities|Casting|CastToGrid_Object_Parent Actor))
    (bind _returnvalue (Game|SpawnActorfromClass "/Game/OurStuff/Blueprints/Whistle2.Whistle2_C" (Math|Conversions|ToTransform(Vector) (Transformation|GetActorLocation _asgrid_object_parent)) "Undefined" 0 0))
    (Rendering|SetVisibility (Variables|Default|GetParticleSystem) true false)
    (Variables|Default|SetUsed true)))

(event Custom|Start
  (Utilities|Casting|CastToStudent (Pawn|GetControlledPawn (Game|GetPlayerController 0))
    (:then
      (Rendering|SetVisibility (Variables|Default|GetStaticMesh) false true))
    (:CastFailed
      (Rendering|SetVisibility (Variables|Default|GetStaticMesh) true true))))

(event Custom|DestroyTrap
  (bind _trappedkid (Variables|Default|GetTrappedKid))
  (Utilities|IsValid _trappedkid
    (:Is%20Valid
      (Rendering|SetOnlyOwnerSee _trappedkid true :!class /Script/Engine.PrimitiveComponent)
      (if (Variables|Default|GetUsed)
        (Actor|DestroyActor)))))

(event EventBeginPlay
  (CallFunction|Start))

(event EventNotifyDPSTurnPassed
  (CallFunction|DestroyTrap))

(fn ConstructionScript)
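; DPS is the seeker pawn in turn-based hide-and-seek, capturing players who overlap its view range and revealing Student meshes inside its vision.
; Each turn it gains action points from the game mode, restores movement and refreshes text allowance.
; Action points pay for traps, super traps (same Trap class) and backup.
; Backup spawns near HQ, always as Back_Up1, takes control, and later hands possession back, ending the turn if points are spent.
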(event OnComponentEndOverlap(Vision)
  (params (OverlappedComponent :type Primitive%20Component%20Object%20Reference) (OtherActor :type Actor%20Object%20Reference) (OtherComp :type Primitive%20Component%20Object%20Reference) (OtherBodyIndex :type Integer))
  (bind _asstudent (Utilities|Casting|CastToStudent OtherActor))
  (Rendering|SetOnlyOwnerSee (Variables|/Game/OurStuff/Blueprints/Player/HideAndSeekPlayer.HideAndSeekPlayer_C|GetPlayerMesh _asstudent) true :!class /Script/Engine.PrimitiveComponent))

(event OnComponentBeginOverlap(WalkingCollision)
  (params (OverlappedComponent :type Primitive%20Component%20Object%20Reference) (OtherActor :type Actor%20Object%20Reference) (OtherComp :type Primitive%20Component%20Object%20Reference) (OtherBodyIndex :type Integer) (bFromSweep :type Boolean) (SweepResult :type Hit%20Result%20Structure%20%28by%20ref%29)))

(event OnComponentBeginOverlap(ViewRange)
  (params (OverlappedComponent :type Primitive%20Component%20Object%20Reference) (OtherActor :type Actor%20Object%20Reference) (OtherComp :type Primitive%20Component%20Object%20Reference) (OtherBodyIndex :type Integer) (bFromSweep :type Boolean) (SweepResult :type Hit%20Result%20Structure%20%28by%20ref%29))
  (bind _ashide_and_seek_player (Utilities|Casting|CastToHideAndSeekPlayer OtherActor))
  (Default|GetCaptured _ashide_and_seek_player))

(event OnComponentBeginOverlap(Vision)
  (params (OverlappedComponent :type Primitive%20Component%20Object%20Reference) (OtherActor :type Actor%20Object%20Reference) (OtherComp :type Primitive%20Component%20Object%20Reference) (OtherBodyIndex :type Integer) (bFromSweep :type Boolean) (SweepResult :type Hit%20Result%20Structure%20%28by%20ref%29))
  (bind _asstudent (Utilities|Casting|CastToStudent OtherActor))
  (Rendering|SetOnlyOwnerSee (Variables|/Game/OurStuff/Blueprints/Player/HideAndSeekPlayer.HideAndSeekPlayer_C|GetPlayerMesh _asstudent) false :!class /Script/Engine.PrimitiveComponent))

(event Custom|TurnBegins
  (bind _backup (Variables|Default|GetBackup))
  ;[1 1 1] Handle what occurs at the beginning of a turn
  (bind _ashide_and_seek_game_mode (Utilities|Casting|CastToHideAndSeekGameMode (Game|GetGameMode)))
  (CallFunction|AddAP (Variables|/Game/OurStuff/HideAndSeekGameMode.HideAndSeekGameMode_C|GetDPSAPIncreasePerTurn _ashide_and_seek_game_mode))
  (Variables|Default|SetisMovementEnabled true)
  (Variables|Default|SetshouldBeAbleToMoveAfterMovement true)
  (CallFunction|RefreshTexts)
  (Utilities|IsValid _backup
    (:Is%20Valid
      (Variables|/Game/OurStuff/Blueprints/Player/HideAndSeekPlayer.HideAndSeekPlayer_C|SetmovementPoints _backup (Variables|Default|GetBackupMovementPoints)))))

(event Custom|placeTrap
  (params (NewParam :type Gameplay%20PC%20Object%20Reference))
  (bind _action_success (CallFunction|PlaceTrapAction))
  (if _action_success
    (Game|SpawnActorfromClass "/Game/OurStuff/Blueprints/Trap.Trap_C" (Math|Conversions|ToTransform(Vector) (Transformation|GetWorldLocation (Variables|/Game/OurStuff/Blueprints/Grid_Object_Parent.Grid_Object_Parent_C|GetGridAnchor (.AsHide%20and%20Seek%20Player (Utilities|Casting|CastToHideAndSeekPlayer (Pawn|GetControlledPawn NewParam)))))) "AlwaysSpawn" 0 0)))

(event Custom|PlaceSuperTrap
  (params (PC :type Gameplay%20PC%20Object%20Reference))
  (bind _action_success (CallFunction|SuperTrapAction))
  (if _action_success
    (Game|SpawnActorfromClass "/Game/OurStuff/Blueprints/Trap.Trap_C" (Math|Conversions|ToTransform(Vector) (Transformation|GetWorldLocation (Variables|/Game/OurStuff/Blueprints/Grid_Object_Parent.Grid_Object_Parent_C|GetGridAnchor (.AsStudent (Utilities|Casting|CastToStudent (Pawn|GetControlledPawn (Game|GetPlayerController 0))))))) "AlwaysSpawn" 0 0)))

(event Custom|refreshTexts
  (bind _asgameplay_pc (Utilities|Casting|CastToGameplayPC (Game|GetPlayerController 0)))
  (Variables|/Game/Blueprints/GamePlay/GameplayPC.GameplayPC_C|SettextsAvailable _asgameplay_pc (Variables|/Game/Blueprints/GamePlay/GameplayPC.GameplayPC_C|GettextsReceivedEachRound _asgameplay_pc)))

(event Custom|TurnEnded
  (bind _wasdeleted (Default|TurnEnded (Variables|Default|GetBackup)))
  (if _wasdeleted
    (Variables|Default|SethasActiveBackup false)))

(event Custom|RepossessEvent
  (Pawn|Possess (Pawn|GetController (Variables|Default|GetBackup)) self)
  (Variables|Default|SetisMovementEnabled false)
  (Utilities|FlowControl|Delay 0.5)
  (bind _ashide_and_seek_game_mode (Utilities|Casting|CastToHideAndSeekGameMode (Game|GetGameMode)))
  (if (not (Variables|/Game/OurStuff/HideAndSeekGameMode.HideAndSeekGameMode_C|GetisStudentsTurn _ashide_and_seek_game_mode))
    (Variables|Default|SetisMovementEnabled true)
    (if (<= (Variables|Default|GetAP) 0)
      (bind _ashide_and_seek_game_mode_2 (Utilities|Casting|CastToHideAndSeekGameMode (Game|GetGameMode)))
      (Default|ForceEndTurn _ashide_and_seek_game_mode_2 0 self))))

(event Custom|TakeControlOfBackup
  (bind _backup (Variables|Default|GetBackup))
  (Utilities|IsValid _backup
    (:Is%20Valid
      (Default|TakeControl _backup self))))

(event EventBeginPlay)

(fn ConstructionScript
  (|CallParentFunction))

(fn CallBackupAction
  (Utilities|IsValid (Variables|Default|GetBackup)
    (:Is%20Not%20Valid
      (bind _hasenoughactionpoints (CallFunction|HasEnoughActionPoints (Variables|Default|GetcallBackupCost)))
      (if _hasenoughactionpoints
        (Variables|Default|SetAP (- (Variables|Default|GetAP) (Variables|Default|GetcallBackupCost)))
        (bind _outactors (Actor|GetAllActorsOfClass "/Game/OurStuff/Blueprints/Buildings/HQ.HQ_C"))
        (bind _worldlocation (Default|GetTileLocationfromIndex (Variables|/Game/OurStuff/Blueprints/Grid_Object_Parent.Grid_Object_Parent_C|Getgrid (Utilities|Array|Get(acopy) _outactors)) (Variables|/Game/OurStuff/Blueprints/Buildings/HQ.HQ_C|GetfrontOfDPS (Utilities|Array|Get(acopy) _outactors))))
        (if (== (Math|Random|RandomIntegerinRange 0 1) 0)
          _
          (else
            _))
        (bind _returnvalue (Game|SpawnActorfromClass "/Game/OurStuff/Blueprints/Player/BackUp/Back_Up1.Back_Up1_C" (Math|Conversions|ToTransform(Vector) _worldlocation) "Undefined" 0 0))
        (bind _output_get (Variables|Default|SetBackup _returnvalue))
        (Variables|/Game/OurStuff/Blueprints/Grid_Object_Parent.Grid_Object_Parent_C|Setgrid _output_get (Variables|Default|Getgrid))
        (Variables|/Game/OurStuff/Blueprints/Grid_Object_Parent.Grid_Object_Parent_C|Setindex _output_get (Variables|Default|Getindex))
        (Variables|/Game/OurStuff/Blueprints/Player/HideAndSeekPlayer.HideAndSeekPlayer_C|SetAP _output_get 0)
        (Variables|/Game/OurStuff/Blueprints/Player/HideAndSeekPlayer.HideAndSeekPlayer_C|SetmovementPoints _output_get (Variables|Default|GetBackupMovementPoints))
        (Variables|Default|SethasActiveBackup true)
        (CallFunction|TakeControlOfBackup)))))

(fn CommandBackupAction
  (bind _hasenoughactionpoints (CallFunction|HasEnoughActionPoints (Variables|Default|GetcommandBackupCost)))
  (if _hasenoughactionpoints
    (Variables|Default|SetAP (- (Variables|Default|GetAP) (Variables|Default|GetcommandBackupCost)))
    (CallFunction|TakeControlOfBackup)))

(fn PlaceTrapAction
  (bind _hasenoughactionpoints (CallFunction|HasEnoughActionPoints (Variables|Default|GetplaceTrapCost)))
  (if _hasenoughactionpoints
    (Variables|Default|SetAP (- (Variables|Default|GetAP) (Variables|Default|GetplaceTrapCost)))
    (return true)
    (else
      (return false))))

(fn ChangeAp
  (params (ap%20added :type Integer))
  (Variables|Default|SetAP (+ (Variables|Default|GetAP) ap%20added)))

(fn SuperTrapAction
  (bind _hasenoughactionpoints (CallFunction|HasEnoughActionPoints (Variables|Default|GetheatSeekingCost)))
  (if _hasenoughactionpoints
    (Variables|Default|SetAP (- (Variables|Default|GetAP) (Variables|Default|GetheatSeekingCost)))
    (return true)
    (else
      (return false))))

(fn Reposses
  (CallFunction|RepossessEvent))
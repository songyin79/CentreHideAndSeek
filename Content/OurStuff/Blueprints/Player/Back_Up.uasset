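; Back_Up is a turn-limited backup pawn that the DPS pawn's controller can possess, capturing any HideAndSeekPlayer overlapping its Box or ViewRange.
; TakeControl stores the DPS pawn and hands its controller to the backup, which starts with one movement point.
; Ending a turn returns control to DPS, and TurnEnded destroys the backup once its lifetime in turns is reached.
; HUD backup-flag clearing exists only in disconnected nodes.
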(event OnComponentBeginOverlap(ViewRange)
  (params (OverlappedComponent :type Primitive%20Component%20Object%20Reference) (OtherActor :type Actor%20Object%20Reference) (OtherComp :type Primitive%20Component%20Object%20Reference) (OtherBodyIndex :type Integer) (bFromSweep :type Boolean) (SweepResult :type Hit%20Result%20Structure%20%28by%20ref%29))
  (bind _ashide_and_seek_player (Utilities|Casting|CastToHideAndSeekPlayer OtherActor))
  (Default|GetCaptured _ashide_and_seek_player))

(event OnComponentBeginOverlap(Box)
  (params (OverlappedComponent :type Primitive%20Component%20Object%20Reference) (OtherActor :type Actor%20Object%20Reference) (OtherComp :type Primitive%20Component%20Object%20Reference) (OtherBodyIndex :type Integer) (bFromSweep :type Boolean) (SweepResult :type Hit%20Result%20Structure%20%28by%20ref%29))
  (bind _ashide_and_seek_player (Utilities|Casting|CastToHideAndSeekPlayer OtherActor))
  (Default|GetCaptured _ashide_and_seek_player))

(event EventBeginPlay
  (Variables|Default|SetmaxMovementPoints 1))

(event EventTurnMustEnd
  (Default|Reposses (Variables|Default|GetDPS)))

(event EventTick
  (params (DeltaSeconds :type Float%20%28single-precision%29)))

(fn ConstructionScript
  (|CallParentFunction))

(fn DeleteItself
  (bind _returnvalue (Game|GetPlayerController 0))
  (Utilities|IsValid _returnvalue
    (:Is%20Valid
      (Pawn|Possess _returnvalue (Variables|Default|GetDPS))
      (Actor|DestroyActor self)
      ;[1 1 1] Update HUD?
      (bind _returnvalue_2 (Settings|GetGameUserSettings)))))

(fn TakeControl
  (params (DPS :type DPS%20Object%20Reference))
  (bind _output_get (Variables|Default|SetDPS DPS))
  (Pawn|Possess (Pawn|GetController _output_get) self))

(fn TurnEnded
  (Default|Reposses (Variables|Default|GetDPS))
  (bind _result (Math|Integer|IncrementInt (Variables|Default|GetturnsHasBeenAliveFor))
    (:%20%20
      (if (>= _result (Variables|Default|GetlifetimeInTurns))
        (CallFunction|DeleteItself)
        (return true)
        (else
          (return false))))))

(fn GoBacktoDPSPawn
  (Default|Reposses (Variables|Default|GetDPS)))
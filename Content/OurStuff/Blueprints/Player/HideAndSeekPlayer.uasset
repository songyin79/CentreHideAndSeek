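; Base player pawn for a turn-based hide-and-seek game, moving one grid tile at a time on action and movement points.
; MoveAction pays the cost or delegates HQ and objective exits; axis helpers pick the target tile, crossing between grids.
; MovePlayer checks objects, objectives and buildings, handing entries to objectives or HQ, with Spectators skipping checks.
; Timelines smooth movement and rotation, and exhausted points end the turn through the game mode.
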(event Custom|Delay
  (Utilities|FlowControl|Delay 0.75))

(event Custom|Rotate
  (params (rotation :type Rotator))
  (bind (_roll _pitch _yaw) (Math|Rotator|BreakRotator rotation))
  ;[1 0.009923 0.03977] Rotate the player smoothly
  (bind _output_get (Variables|Default|Setrotation (Transformation|GetActorRotation)))
  (if (Math|Float|NearlyEqual(Float) (.Yaw (Math|Rotator|BreakRotator _output_get)) -1.8e+02 1.0)
    (Variables|Default|Setrotation (Math|Rotator|MakeRotator (.Roll (Math|Rotator|BreakRotator _output_get)) (.Pitch (Math|Rotator|BreakRotator _output_get)) 1.8e+02))
    (bind _rotationscalar (Timeline|RotationTimeline PlayFromStart)
      (:Update
        (Transformation|SetActorRotation (Math|Rotator|MakeRotator (+ (* _rotationscalar (- _roll (.Roll (Math|Rotator|BreakRotator (Variables|Default|Getrotation))))) (.Roll (Math|Rotator|BreakRotator (Variables|Default|Getrotation)))) (+ (* _rotationscalar (- _pitch (.Pitch (Math|Rotator|BreakRotator (Variables|Default|Getrotation))))) (.Pitch (Math|Rotator|BreakRotator (Variables|Default|Getrotation)))) (+ (* _rotationscalar (- _yaw (.Yaw (Math|Rotator|BreakRotator (Variables|Default|Getrotation))))) (.Yaw (Math|Rotator|BreakRotator (Variables|Default|Getrotation))))))))
    (else
      (Timeline|RotationTimeline PlayFromStart))))

(event Custom|Move
  (params (initPosition :type Vector) (endPosition :type Vector))
  (bind _movementtimeline (Variables|Default|GetMovementTimeline))
  ;[0.1915 0.09994 1] Move the player between two points smoothly
  (Variables|Default|SetisMovementEnabled false)
  (CallFunction|EnterMovement)
  (Components|Timeline|SetPlayRate _movementtimeline (/ 1.0 (Variables|Default|GetrunTime)))
  (Components|Timeline|PlayfromStart _movementtimeline))

(event Custom|RemoveAbility
  (Variables|Default|SetmovementPoints 0)
  (Variables|Default|SetisMovementEnabled false)
  (Variables|Default|SetshouldBeAbleToMoveAfterMovement false))

(event EventBeginPlay
  (if (Variables|Default|GetInvisibile)
    (Rendering|SetOnlyOwnerSee (Variables|Default|GetPlayerMesh) true :!class /Script/Engine.PrimitiveComponent)))

(fn ConstructionScript
  (|CallParentFunction))

(fn MovePlayer
  (params (tileIndex :type Integer) (isEnteringObjective :type Boolean))
  (Utilities|Casting|CastToSpectator self
    (:then
      ;[0.4545 0.1085 1] If the tile is unoccupied, move the player to that location
      (Math|Integer|DecrementInt (Variables|Default|GetmovementPoints) :!label _label
        (:%20%20
          (bind _worldlocation (Default|GetTileLocationfromIndex (Variables|Default|Getgrid) tileIndex))
          (CallFunction|Rotate (Math|Rotator|MakeRotator 0.0 0.0 (.Yaw (Math|Rotator|BreakRotator (Math|Rotator|FindLookatRotation (Transformation|GetActorLocation) (Math|Vector|MakeVector (.X (Math|Vector|BreakVector _worldlocation)) (.Y (Math|Vector|BreakVector _worldlocation)) (+ (.Z (Math|Vector|BreakVector _worldlocation)) (Variables|/Game/OurStuff/Blueprints/TileSection.TileSection_C|GetsizeOfMeshZ (Variables|Default|Getgrid)))))))))
          (CallFunction|Move (Transformation|GetActorLocation) (Math|Vector|MakeVector (.X (Math|Vector|BreakVector _worldlocation)) (.Y (Math|Vector|BreakVector _worldlocation)) (+ (.Z (Math|Vector|BreakVector _worldlocation)) (Variables|/Game/OurStuff/Blueprints/TileSection.TileSection_C|GetsizeOfMeshZ (Variables|Default|Getgrid)))))
          (Variables|Default|Setindex tileIndex)
          (if (and (== (Variables|Default|GetAP) 0) (== (Variables|Default|GetmovementPoints) 0))
            (CallFunction|TurnMustEnd))
          (return true))))
    (:CastFailed
      (if isEnteringObjective
        (goto _label)
        (else
          ;[0.9997 1 0.06198] Check to see if there is already an object or an objective where we are trying to move
          (bind _isindextaken (Default|CheckifIndexIsTakenbyAnObject (Variables|Default|Getgrid) tileIndex))
          (if _isindextaken
            ;[1 0 0.01891] If there is an object, a building, or an objective that can't be entered at the index, prevent the player from moving
            (Utilities|Casting|CastToBack_Up self :!label _label_2
              (:then
                _)
              (:CastFailed
                (if (== (Variables|Default|GetmovementPoints) 1)
                  (Math|Integer|IncrementInt (Variables|Default|GetAP)
                    (:%20%20
                      (Math|Integer|DecrementInt (Variables|Default|GetmovementPoints)
                        (:%20%20
                          _)))))))
            (bind _grid (CallFunction|FindGridCorrelatingtoAWorldLocation (Transformation|GetActorLocation)))
            (Variables|Default|Setgrid _grid)
            (return false)
            (else
              (bind (_iswithinobjective _objective) (Default|CheckifIndexIsinAnObjective (Variables|Default|Getgrid) tileIndex))
              (if _iswithinobjective
                ;[0.2573 1 0.1697] See if the player is a student and, if they are, see if the objective can be entered by a student
                (Utilities|Casting|CastToStudent self
                  (:then
                    (if (Variables|/Game/OurStuff/Blueprints/Objective.Objective_C|GetcanObjectiveBeEnteredByAStudent _objective)
                      ;[0.212 1 0.6823] Try to move the player into the objective by delegating movement to the obective
                      (bind _successfullyentered (Default|StudentIsAttemptingtoEnterObjective _objective self))
                      (if _successfullyentered
                        (Math|Integer|DecrementInt (Variables|Default|GetmovementPoints))
                        (else
                          (goto _label_2)))
                      (else
                        (goto _label_2))))
                  (:CastFailed
                    ;[1 0.2602 0.659] If the player entering is not a student, try to enter
                    (bind _asdps (Utilities|Casting|CastToDPS self))
                    (bind (_student _isobjectiveoccupied _successfulyentered) (Default|DPSIsEnteringObjective _objective _asdps))
                    (if _successfulyentered
                      (Math|Integer|DecrementInt (Variables|Default|GetmovementPoints)
                        (:%20%20
                          (CallFunction|GetCaptured _student)))
                      (else
                        (goto _label_2)))))
                (else
                  ;[1 0.9084 0.1042] Check if the index is taken by a building
                  (bind (_iswithinobjective_2 _building) (Default|CheckifIndexIsTakenbyBuilding (Variables|Default|Getgrid) tileIndex))
                  (if _iswithinobjective_2
                    ;[0 1 0.001442] If the Building was HQ, delegate movement to HQ
                    (bind _ashq (Utilities|Casting|CastToHQ _building)
                      (:then
                        (Default|PlayerIsEnteringHQ _ashq self))
                      (:CastFailed
                        (goto _label_2)))
                    (else
                      (goto _label))))))))))))

(fn MoveAction
  (params (moveDirection :type Boolean) (scale :type Float%20%28single-precision%29))
  (if (and (or (== scale 1.0) (== scale -1.0)) (Variables|Default|GetisMovementEnabled))
    (Utilities|Casting|CastToSpectator self
      (:then
        (if moveDirection :!label _label
          (CallFunction|MoveAlongYAxis scale)
          (else
            (CallFunction|MoveAlongXAxis scale)))
        (return true))
      (:CastFailed
        (if (Variables|Default|GetisInHQ)
          (bind _outactors (Actor|GetAllActorsOfClass "/Game/OurStuff/Blueprints/Buildings/HQ.HQ_C"))
          (Default|PlayerIsExitingHQ (Utilities|Array|Get(acopy) _outactors) self)
          (elif (Variables|Default|GetisWithinAnObjective)
            ;[0.2789 1 0.2634] If movement is not enabled and the player is in an objective, delegate to the objective movement
            (Utilities|Casting|CastToStudent self
              (:then
                (Default|StudentIsExitingObjective (Variables|Default|GetobjectivePlayerIsIn)))
              (:CastFailed
                (Default|DPSIsExitingObjective (Variables|Default|GetobjectivePlayerIsIn) self)))
            (CallFunction|Delay)
            (else
              (if (Variables|Default|GetisHidden)
                (LocalVariables|SetCost (Variables|Default|GetcostOfMovingWhileHidden))
                (else
                  (LocalVariables|SetCost (Variables|Default|GetmovementCost))))
              (if (> (Variables|Default|GetmovementPoints) 0)
                (goto _label)
                (else
                  ;[1 0.03692 0.6606] Adjust action points as necessary
                  (bind _hasenoughactionpoints (CallFunction|HasEnoughActionPoints (LocalVariables|GetCost)))
                  (if _hasenoughactionpoints
                    (Variables|Default|SetAP (- (Variables|Default|GetAP) (LocalVariables|GetCost)))
                    (Variables|Default|SetmovementPoints 1)
                    (goto _label)
                    (else
                      (return false))))))))))))

(fn HasEnoughActionPoints
  (params (actionCost :type Integer))
  (return (>= (Variables|Default|GetAP) actionCost)))

(fn MoveAlongXAxis
  (params (scale :type Float%20%28single-precision%29))
  (if (== scale 1.0)
    ;[1 0.1591 0.832] Move Right
    (bind _iswithingrid (CallFunction|IsWithinRangeOfGrid (+ (Transformation|GetActorLocation) (Math|Vector|MakeVector (Variables|/Game/OurStuff/Blueprints/TileSection.TileSection_C|GetsizeOfMeshX (Variables|Default|Getgrid)) 0.0 0.0)) (Variables|Default|Getgrid)))
    (if _iswithingrid
      (LocalVariables|SetmoveToLocation (+ (Variables|Default|Getindex) 1))
      (Variables|Default|SetfacingDirection 0 :!label _label)
      (CallFunction|MovePlayer (LocalVariables|GetmoveToLocation) false)
      (else
        (bind (_grid _foundvalidgrid) (CallFunction|FindGridCorrelatingtoAWorldLocation (+ (Transformation|GetActorLocation) (Math|Vector|MakeVector (Variables|/Game/OurStuff/Blueprints/TileSection.TileSection_C|GetsizeOfMeshX (Variables|Default|Getgrid)) 0.0 0.0))))
        (if _foundvalidgrid
          (Variables|Default|Setgrid _grid)
          (bind _index (CallFunction|ConvertWorldLocationtoIndexforMovement (+ (Transformation|GetActorLocation) (Math|Vector|MakeVector (Variables|/Game/OurStuff/Blueprints/TileSection.TileSection_C|GetsizeOfMeshX (Variables|Default|Getgrid)) 0.0 0.0))))
          (bind _output_get (Variables|Default|Setindex _index))
          (LocalVariables|SetmoveToLocation _output_get)
          (goto _label))))
    (else
      ;[0.1302 1 0.03963] Move Left
      (if (== scale -1.0)
        (bind _iswithingrid_2 (CallFunction|IsWithinRangeOfGrid (- (Transformation|GetActorLocation) (Math|Vector|MakeVector (Variables|/Game/OurStuff/Blueprints/TileSection.TileSection_C|GetsizeOfMeshX (Variables|Default|Getgrid)) 0.0 0.0)) (Variables|Default|Getgrid)))
        (if _iswithingrid_2
          (LocalVariables|SetmoveToLocation (- (Variables|Default|Getindex) 1))
          (Variables|Default|SetfacingDirection 1 :!label _label_2)
          (CallFunction|MovePlayer (LocalVariables|GetmoveToLocation) false)
          (else
            (bind (_grid_2 _foundvalidgrid_2) (CallFunction|FindGridCorrelatingtoAWorldLocation (- (Transformation|GetActorLocation) (Math|Vector|MakeVector (Variables|/Game/OurStuff/Blueprints/TileSection.TileSection_C|GetsizeOfMeshX (Variables|Default|Getgrid)) 0.0 0.0))))
            (if _foundvalidgrid_2
              (Variables|Default|Setgrid _grid_2)
              (bind _index_2 (CallFunction|ConvertWorldLocationtoIndexforMovement (- (Transformation|GetActorLocation) (Math|Vector|MakeVector (Variables|/Game/OurStuff/Blueprints/TileSection.TileSection_C|GetsizeOfMeshX (Variables|Default|Getgrid)) 0.0 0.0))))
              (bind _output_get_2 (Variables|Default|Setindex _index_2))
              (LocalVariables|SetmoveToLocation _output_get_2)
              (goto _label_2))))))))

(fn MoveAlongYAxis
  (params (scale :type Float%20%28single-precision%29))
  (bind _returnvalue (Transformation|GetActorLocation))
  (bind _x (Math|Vector|BreakVector _returnvalue))
  (if (== scale 1.0)
    ;[0.2724 0.09082 1] Move In positive direction
    ;;[0.01435 1 0.006423] Is where I want to go in this grid?
    (bind _iswithingrid (CallFunction|IsWithinRangeOfGrid (+ (Transformation|GetActorLocation) (Math|Vector|MakeVector 0.0 (Variables|/Game/OurStuff/Blueprints/TileSection.TileSection_C|GetsizeOfMeshY (Variables|Default|Getgrid)) 0.0)) (Variables|Default|Getgrid)))
    (if _iswithingrid
      (LocalVariables|SetmoveToLocation (+ (Variables|/Game/OurStuff/Blueprints/TileSection.TileSection_C|GettilesInXDirection (Variables|Default|Getgrid)) (Variables|Default|Getindex)))
      (Variables|Default|SetfacingDirection 2 :!label _label)
      (CallFunction|MovePlayer (LocalVariables|GetmoveToLocation) false)
      (else
        ;;[1 0.2268 0] If its not, find the next grid and move within there
        (bind (_grid _foundvalidgrid) (CallFunction|FindGridCorrelatingtoAWorldLocation (+ (Transformation|GetActorLocation) (Math|Vector|MakeVector 0.0 (Variables|/Game/OurStuff/Blueprints/TileSection.TileSection_C|GetsizeOfMeshY (Variables|Default|Getgrid)) 0.0))))
        (if _foundvalidgrid
          (Variables|Default|Setgrid _grid)
          (bind _index (CallFunction|ConvertWorldLocationtoIndexforMovement (+ (Transformation|GetActorLocation) (Math|Vector|MakeVector 0.0 (Variables|/Game/OurStuff/Blueprints/TileSection.TileSection_C|GetsizeOfMeshY (Variables|Default|Getgrid)) 0.0))))
          (bind _worldlocation (Default|GetTileLocationfromIndex (Variables|Default|Getgrid) _index))
          (if (Math|Float|NearlyEqual(Float) (.X (Math|Vector|BreakVector _worldlocation)) (.X (Math|Vector|BreakVector (+ (Transformation|GetActorLocation) (Math|Vector|MakeVector 0.0 (Variables|/Game/OurStuff/Blueprints/TileSection.TileSection_C|GetsizeOfMeshY (Variables|Default|Getgrid)) 0.0)))) 1e-06)
            (LocalVariables|SetmoveToLocation _index)
            (goto _label)
            (else
              (LocalVariables|SetmoveToLocation (+ _index (Math|Float|Truncate (/ (- (.X (Math|Vector|BreakVector _worldlocation)) (.X (Math|Vector|BreakVector (+ (Transformation|GetActorLocation) (Math|Vector|MakeVector 0.0 (Variables|/Game/OurStuff/Blueprints/TileSection.TileSection_C|GetsizeOfMeshY (Variables|Default|Getgrid)) 0.0))))) (Variables|/Game/OurStuff/Blueprints/TileSection.TileSection_C|GetsizeOfMeshX (Variables|Default|Getgrid))))))
              (goto _label))))))
    (else
      ;[0.2172 1 0.2027] Move in negative direction
      (if (== scale -1.0)
        (bind _iswithingrid_2 (CallFunction|IsWithinRangeOfGrid (- _returnvalue (Math|Vector|MakeVector 0.0 (Variables|/Game/OurStuff/Blueprints/TileSection.TileSection_C|GetsizeOfMeshY (Variables|Default|Getgrid)) 0.0)) (Variables|Default|Getgrid)))
        (if _iswithingrid_2
          (LocalVariables|SetmoveToLocation (- (Variables|Default|Getindex) (Variables|/Game/OurStuff/Blueprints/TileSection.TileSection_C|GettilesInXDirection (Variables|Default|Getgrid))))
          (Variables|Default|SetfacingDirection 3 :!label _label_2)
          (CallFunction|MovePlayer (LocalVariables|GetmoveToLocation) false)
          (else
            (bind (_grid_2 _foundvalidgrid_2) (CallFunction|FindGridCorrelatingtoAWorldLocation (- _returnvalue (Math|Vector|MakeVector 0.0 (Variables|/Game/OurStuff/Blueprints/TileSection.TileSection_C|GetsizeOfMeshY (Variables|Default|Getgrid)) 0.0))))
            (if _foundvalidgrid_2
              (Variables|Default|Setgrid _grid_2)
              (bind _index_2 (CallFunction|ConvertWorldLocationtoIndexforMovement (- _returnvalue (Math|Vector|MakeVector 0.0 (Variables|/Game/OurStuff/Blueprints/TileSection.TileSection_C|GetsizeOfMeshY (Variables|Default|Getgrid)) 0.0))))
              (bind _worldlocation_2 (Default|GetTileLocationfromIndex (Variables|Default|Getgrid) _index_2))
              (if (Math|Float|NearlyEqual(Float) (.X (Math|Vector|BreakVector _worldlocation_2)) _x 1e-06)
                (bind _output_get (Variables|Default|Setindex _index_2))
                (LocalVariables|SetmoveToLocation _output_get)
                (goto _label_2)
                (else
                  (bind _output_get_2 (Variables|Default|Setindex (+ _index_2 (Math|Float|Round (/ (- (.X (Math|Vector|BreakVector _worldlocation_2)) _x) (Variables|/Game/OurStuff/Blueprints/TileSection.TileSection_C|GetsizeOfMeshX (Variables|Default|Getgrid)))))))
                  (LocalVariables|SetmoveToLocation _output_get_2)
                  (goto _label_2))))))))))

(fn GetCaptured)

(fn EnterMovement)

(fn ExitMovement)

(fn AddAP
  (params (IncomingAP :type Integer))
  (bind _maxap (Variables|Default|GetMaxAP))
  (bind _output_get (Variables|Default|SetAP (+ IncomingAP (Variables|Default|GetAP))))
  (if (>= _output_get _maxap)
    (Variables|Default|SetAP _maxap)))

(fn TurnMustEnd
  (bind _ashide_and_seek_game_mode (Utilities|Casting|CastToHideAndSeekGameMode (Game|GetGameMode)))
  (Default|ForceEndTurn _ashide_and_seek_game_mode 0 self))

(fn CheckifIndexIsAvailable
  (params (index :type Integer))
  (return false))

(fn LookatFacingDirection
  (params (directionToFace :type Integer))
  (bind _returnvalue (Transformation|GetActorLocation))
  (bind _grid (Variables|Default|Getgrid))
  (bind _sizeofmeshx (Variables|/Game/OurStuff/Blueprints/TileSection.TileSection_C|GetsizeOfMeshX _grid))
  (bind _sizeofmeshy (Variables|/Game/OurStuff/Blueprints/TileSection.TileSection_C|GetsizeOfMeshY _grid))
  (bind _returnvalue_2 (Math|Vector|MakeVector _sizeofmeshx 0.0 0.0))
  (bind _returnvalue_3 (Math|Vector|MakeVector 0.0 _sizeofmeshy 0.0))
  (bind _output_get (Variables|Default|SetfacingDirection directionToFace))
  (if (== _output_get 0)
    (Transformation|SetActorRotation (Math|Rotator|FindLookatRotation _returnvalue (+ _returnvalue _returnvalue_2)))
    (elif (== (Variables|Default|GetfacingDirection) 1)
      (Transformation|SetActorRotation (Math|Rotator|FindLookatRotation _returnvalue (- _returnvalue _returnvalue_2)))
      (elif (== (Variables|Default|GetfacingDirection) 2)
        (Transformation|SetActorRotation (Math|Rotator|FindLookatRotation _returnvalue (+ _returnvalue _returnvalue_3)))
        (elif (== (Variables|Default|GetfacingDirection) 2)
          (Transformation|SetActorRotation (Math|Rotator|FindLookatRotation _returnvalue (- _returnvalue _returnvalue_3))))))))
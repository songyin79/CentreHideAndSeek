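; Student is the hider pawn in a turn-based, grid-based hide-and-seek game, spending action points on running, whistling, texting and objectives.
; Running repeats MoveAction along the facing direction with a temporarily swapped RunTime; whistling spawns an actor registered with the game mode.
; First capture teleports the student to HQ's tile and disables movement; a second removes them from play.
; Captures raise DPS score through an authority-checked game mode call, and overlap events toggle owner-only mesh visibility.
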(event OnComponentBeginOverlap(Box)
  (params (OverlappedComponent :type Primitive%20Component%20Object%20Reference) (OtherActor :type Actor%20Object%20Reference) (OtherComp :type Primitive%20Component%20Object%20Reference) (OtherBodyIndex :type Integer) (bFromSweep :type Boolean) (SweepResult :type Hit%20Result%20Structure%20%28by%20ref%29))
  (Rendering|SetOnlyOwnerSee (Variables|Default|GetPlayerMesh) false :!class /Script/Engine.PrimitiveComponent))

(event OnComponentEndOverlap(PlayerMesh)
  (params (OverlappedComponent :type Primitive%20Component%20Object%20Reference) (OtherActor :type Actor%20Object%20Reference) (OtherComp :type Primitive%20Component%20Object%20Reference) (OtherBodyIndex :type Integer))
  (Rendering|SetOnlyOwnerSee (Variables|Default|GetPlayerMesh) true :!class /Script/Engine.PrimitiveComponent))

(event Custom|Whistle
  ;[1 1 1] JAMES CHANGED THIS IF TRAPS ARENT PLACED PROPERLY
  (bind _action_success (CallFunction|WhistleAction))
  (if _action_success
    (bind _returnvalue (Game|SpawnActorfromClass "/Game/OurStuff/Blueprints/Whistle1.Whistle1_C" (Math|Conversions|ToTransform(Vector) (Transformation|GetActorLocation (.AsHide%20and%20Seek%20Player (Utilities|Casting|CastToHideAndSeekPlayer (Pawn|GetControlledPawn (Game|GetPlayerController 0)))))) "AlwaysSpawn" 0 0))
    (Utilities|Array|Add (Variables|/Game/OurStuff/HideAndSeekGameMode.HideAndSeekGameMode_C|GetWhistles (.AsHide%20and%20Seek%20Game%20Mode (Utilities|Casting|CastToHideAndSeekGameMode (Game|GetGameMode)))) _returnvalue)
    (if (== (Variables|Default|GetAP) 0)
      (CallFunction|TurnMustEnd))))

(event Custom|RequestDPSScoreIncrease
  (params (ScoreAmount :type Integer))
  (bind _returnvalue (Game|GetGameMode))
  (Utilities|IsValid _returnvalue
    (:Is%20Valid
      (Networking|SwitchHasAuthority
        (:Authority
          (bind _ashide_and_seek_game_mode (Utilities|Casting|CastToHideAndSeekGameMode _returnvalue))
          (Default|IncreaseDPSScore _ashide_and_seek_game_mode ScoreAmount))))))

(event EventBeginPlay)

(event EventGetCaptured
  ;[1 0.06157 0.1014] Handle the Student being captured
  (if (Variables|Default|GethasBeenCapturedBefore)
    (if (Variables|Default|GetisInGame)
      ;;[1 1 1] Set the player's mesh to a ghost mesh, make it so they can see everyone
      (Variables|Default|SetisInGame false)
      (CallFunction|RequestDPSScoreIncrease (Variables|Default|GetsecondCaptureValue)))
    (else
      (bind _outactors (Actor|GetAllActorsOfClass "/Game/OurStuff/Blueprints/Buildings/HQ.HQ_C"))
      (Variables|Default|SethasBeenCapturedBefore true)
      (bind _output_get (Variables|Default|Setgrid (Variables|/Game/OurStuff/Blueprints/Grid_Object_Parent.Grid_Object_Parent_C|Getgrid (Utilities|Array|Get(acopy) _outactors))))
      (bind _output_get_2 (Variables|Default|Setindex (Variables|/Game/OurStuff/Blueprints/Grid_Object_Parent.Grid_Object_Parent_C|Getindex (Utilities|Array|Get(acopy) _outactors))))
      (bind _worldlocation (Default|GetTileLocationfromIndex _output_get _output_get_2))
      (Transformation|SetActorLocation _worldlocation false false)
      (Variables|Default|SetisMovementEnabled false)
      (Variables|Default|SetisCaptured true)
      (Default|AddStudenttoCapturedStudents (Utilities|Array|Get(acopy) _outactors) self)
      (CallFunction|RequestDPSScoreIncrease (Variables|Default|GetfirstCaptureValue)))))

(fn ConstructionScript
  (|CallParentFunction))

(fn TextAction
  (if (Variables|Default|GetisInGame)
    (bind _hasenoughactionpoints (CallFunction|HasEnoughActionPoints (Variables|Default|GettextCost)))
    (if _hasenoughactionpoints
      (Variables|Default|SetAP (- (Variables|Default|GetAP) (Variables|Default|GettextCost))))))

(fn RunAction
  (bind _facingdirection (Variables|Default|GetfacingDirection))
  (if (Math|Boolean|ANDBoolean (not (Variables|Default|GetisCaptured)) (not (Variables|Default|GetisHidden)) (Variables|Default|GetisMovementEnabled))
    (bind _hasenoughactionpoints (CallFunction|HasEnoughActionPoints (Variables|Default|GetrunCost)))
    (if _hasenoughactionpoints
      (LocalVariables|SetinitRunTime (Variables|Default|GetrunTime))
      (Variables|Default|SetrunTime (Variables|Default|GettimeForRunning))
      (for _index (range 0 4)
        (if (or (not (Variables|Default|GetisTrapped)) (not (Variables|Default|GetisWithinAnObjective)))
          (Variables|Default|SetmovementPoints 100)
          (if (== _facingdirection 0)
            (CallFunction|MoveAction false 1.0)
            (CallFunction|Delay :!label _label)
            (elif (== _facingdirection 1)
              (CallFunction|MoveAction false -1.0)
              (goto _label)
              (elif (== _facingdirection 2)
                (CallFunction|MoveAction true 1.0)
                (goto _label)
                (elif (== _facingdirection 3)
                  (CallFunction|MoveAction true -1.0)
                  (goto _label)))))))
      (Variables|Default|SetrunTime (LocalVariables|GetinitRunTime))
      (Variables|Default|SetmovementPoints 0)
      (Variables|Default|SetAP (- (Variables|Default|GetAP) (Variables|Default|GetrunCost)))
      (if (== (Variables|Default|GetAP) 0)
        (CallFunction|TurnMustEnd))
      (return true)
      (else
        (return false)))))

(fn WhistleAction
  (if (Variables|Default|GetisInGame)
    (bind _hasenoughactionpoints (CallFunction|HasEnoughActionPoints (Variables|Default|GetwhistleCost)))
    (if _hasenoughactionpoints
      (Variables|Default|SetAP (- (Variables|Default|GetAP) (Variables|Default|GetwhistleCost)))
      (return true)
      (else
        (return false)))))

(fn AddAP0
  (params (ap_added :type Integer))
  (Variables|Default|SetAP (+ (Variables|Default|GetAP) ap_added)))

(fn GetObjectiveAction
  (if (Variables|Default|GetisInGame)
    (bind _hasenoughactionpoints (CallFunction|HasEnoughActionPoints (Variables|Default|Getget_Objective_Cost)))
    (if _hasenoughactionpoints
      (Variables|Default|SetAP (- (Variables|Default|GetAP) 1)))))

(fn PerformRun
  (bind _returnvalue (Transformation|GetActorLocation))
  (bind _returnvalue_2 (Transformation|GetActorLocation))
  (bind _returnvalue_3 (Transformation|GetActorLocation))
  (bind _returnvalue_4 (Transformation|GetActorLocation))
  (bind _facingdirection (Variables|Default|GetfacingDirection))
  (bind (_x _y _z) (Math|Vector|BreakVector _returnvalue))
  (bind (_x_2 _y_2 _z_2) (Math|Vector|BreakVector _returnvalue_2))
  (bind (_x_3 _y_3 _z_3) (Math|Vector|BreakVector _returnvalue_3))
  (bind (_x_4 _y_4 _z_4) (Math|Vector|BreakVector _returnvalue_4))
  (Utilities|FlowControl|ForLoopwithBreak 1 5
    (:LoopBody
      (if (== _facingdirection 0)
        (LocalVariables|SetmoveToLocation (Math|Vector|MakeVector (+ (* (Variables|Default|Getindex) (Variables|/Game/OurStuff/Blueprints/TileSection.TileSection_C|GetsizeOfMeshX (Variables|Default|Getgrid))) _x_2) _y_2 _z_2))
        (elif (== _facingdirection 1)
          (LocalVariables|SetmoveToLocation (Math|Vector|MakeVector (- _x_3 (* (Variables|Default|Getindex) (Variables|/Game/OurStuff/Blueprints/TileSection.TileSection_C|GetsizeOfMeshX (Variables|Default|Getgrid)))) _y_3 _z_3))
          (elif (== _facingdirection 2)
            (LocalVariables|SetmoveToLocation (Math|Vector|MakeVector _x_4 (+ (* (Variables|Default|Getindex) (Variables|/Game/OurStuff/Blueprints/TileSection.TileSection_C|GetsizeOfMeshY (Variables|Default|Getgrid))) _y_4) _z_4))
            (elif (== _facingdirection 3)
              (LocalVariables|SetmoveToLocation (Math|Vector|MakeVector _x (- _y (* (Variables|Default|Getindex) (Variables|/Game/OurStuff/Blueprints/TileSection.TileSection_C|GetsizeOfMeshY (Variables|Default|Getgrid)))) _z)))))))))
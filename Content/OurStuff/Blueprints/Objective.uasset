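; Grid-registered objective for a hide-and-seek game that Students occupy to score points and DPS players can enter.
; Players enter from entrance indices and move to the objective's grid index; exits return them to the last entering Student's saved index.
; Turn events count occupancy, then award score through the GameMode on authority, eject the Student and start a cooldown.
; The cooldown only counts down for objectives that allow repeat capture.
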(event OnComponentBeginOverlap(ObjectiveBounds)
  (params (OverlappedComponent :type Primitive%20Component%20Object%20Reference) (OtherActor :type Actor%20Object%20Reference) (OtherComp :type Primitive%20Component%20Object%20Reference) (OtherBodyIndex :type Integer) (bFromSweep :type Boolean) (SweepResult :type Hit%20Result%20Structure%20%28by%20ref%29))
  (if (Utilities|String|Contains (Utilities|GetDisplayName OtherComp) "WalkingCollision" true)
    _))

(event Custom|RequestStudentScoreIncrease
  (bind _returnvalue (Game|GetGameMode))
  (Utilities|IsValid _returnvalue
    (:Is%20Valid
      (Networking|SwitchHasAuthority
        (:Authority
          (bind _ashide_and_seek_game_mode (Utilities|Casting|CastToHideAndSeekGameMode _returnvalue))
          (Utilities|IsValid _ashide_and_seek_game_mode
            (:Is%20Valid
              (Default|IncreaseStudentScore _ashide_and_seek_game_mode (Variables|Default|GetobjectiveValue)))))))))

(event Custom|StudentTurnPassed
  ;[0.0508 1 0] Adjusts variables as necessary when the Students' turns end.
  (if (Variables|Default|GetisObjectiveOccupied)
    (Math|Integer|IncrementInt (Variables|Default|GetturnCounter))
    (elif (Variables|Default|GetcanObectiveBeCapturedMultipleTimes)
      (if (Variables|Default|GetisObjectiveOnCooldown)
        (bind _result (Math|Integer|DecrementInt (Variables|Default|GetturnsUntilObjectiveIsCooledDown))
          (:%20%20
            (if (<= _result 0)
              (Variables|Default|SetisObjectiveOnCooldown false)
              (Variables|Default|SetcanObjectiveBeEnteredByAStudent true)
              (Variables|Default|SetturnCounter 0))))))))

(event Custom|DPSTurnPassed
  ;[1 0.03103 0.05092] Whenever DPS's turn ends, check if the student has been in the objective long enough and, if so, handle it appropriately
  (if (>= (Variables|Default|GetturnCounter) 1)
    (CallFunction|RequestStudentScoreIncrease)
    (CallFunction|StudentIsExitingObjective)
    (Variables|Default|SetturnsUntilObjectiveIsCooledDown (Variables|Default|GetobjectiveCooldown))
    (Variables|Default|SetisObjectiveOnCooldown true)
    (Variables|Default|SetcanObjectiveBeEnteredByAStudent false)
    (Variables|Default|SetturnCounter 0)))

(event EventBeginPlay
  (Default|RegisterObjective (Variables|Default|Getgrid) self))

(fn ConstructionScript
  (|CallParentFunction))

(fn StudentIsAttemptingtoEnterObjective
  (params (Student :type Hide%20and%20Seek%20Player%20Object%20Reference))
  (bind _asstudent (Utilities|Casting|CastToStudent Student))
  (if (Variables|Default|GetcanObjectiveBeEnteredByAStudent)
    (bind _indexisvalid (CallFunction|CheckifPlayerIsonAnEnterIndex (Variables|/Game/OurStuff/Blueprints/Grid_Object_Parent.Grid_Object_Parent_C|Getindex _asstudent)))
    (if _indexisvalid
      (bind _output_get (Variables|Default|SetstudentOccupyingObjective _asstudent))
      (Variables|Default|SetexitIndex (Variables|/Game/OurStuff/Blueprints/Grid_Object_Parent.Grid_Object_Parent_C|Getindex _output_get))
      (CallFunction|MovePlayerEnteringObjective _asstudent)
      (Variables|/Game/OurStuff/Blueprints/Player/HideAndSeekPlayer.HideAndSeekPlayer_C|SetobjectivePlayerIsIn _asstudent self)
      (Variables|/Game/OurStuff/Blueprints/Player/HideAndSeekPlayer.HideAndSeekPlayer_C|SetisWithinAnObjective _asstudent true)
      (Variables|Default|SetisObjectiveOccupied true)
      (Variables|Default|SetcanObjectiveBeEnteredByAStudent false)
      (return true)
      (else
        (return false)))
    (else
      (return false))))

(fn DPSIsEnteringObjective
  (params (DPS :type Hide%20and%20Seek%20Player%20Object%20Reference))
  (bind _indexisvalid (CallFunction|CheckifPlayerIsonAnEnterIndex (Variables|/Game/OurStuff/Blueprints/Grid_Object_Parent.Grid_Object_Parent_C|Getindex DPS)))
  (if _indexisvalid
    (CallFunction|MovePlayerEnteringObjective DPS)
    (Variables|/Game/OurStuff/Blueprints/Player/HideAndSeekPlayer.HideAndSeekPlayer_C|SetobjectivePlayerIsIn DPS self)
    (Variables|/Game/OurStuff/Blueprints/Player/HideAndSeekPlayer.HideAndSeekPlayer_C|SetisWithinAnObjective DPS true)
    (return (Variables|Default|GetstudentOccupyingObjective) (Variables|Default|GetisObjectiveOccupied) true)
    (else
      (return (Variables|Default|GetNULL_STUDENT) false false))))

(fn StudentIsExitingObjective
  (Variables|Default|SetcanObjectiveBeEnteredByAStudent true)
  (Variables|Default|SetisObjectiveOccupied false)
  (Variables|/Game/OurStuff/Blueprints/Player/HideAndSeekPlayer.HideAndSeekPlayer_C|SetisWithinAnObjective (Variables|Default|GetstudentOccupyingObjective) false)
  (CallFunction|MovePlayerExitingObjective (Variables|Default|GetstudentOccupyingObjective))
  (Variables|/Game/OurStuff/Blueprints/Player/HideAndSeekPlayer.HideAndSeekPlayer_C|SetisMovementEnabled (Variables|Default|GetstudentOccupyingObjective) true)
  (Variables|/Game/OurStuff/Blueprints/Player/HideAndSeekPlayer.HideAndSeekPlayer_C|SetobjectivePlayerIsIn (Variables|Default|GetstudentOccupyingObjective) (Variables|Default|GetNULL_OBJECTIVE))
  (Variables|Default|SetstudentOccupyingObjective (Variables|Default|GetNULL_STUDENT))
  (Variables|Default|SetturnCounter 0)
  (return))

(fn MovePlayerEnteringObjective
  (params (Player :type Hide%20and%20Seek%20Player%20Object%20Reference))
  (bind _output_get (Variables|/Game/OurStuff/Blueprints/Grid_Object_Parent.Grid_Object_Parent_C|Setindex Player (Variables|Default|Getindex)))
  (Default|MovePlayer Player _output_get)
  (return "0, 0, 0"))

(fn MovePlayerExitingObjective
  (params (Player :type Hide%20and%20Seek%20Player%20Object%20Reference))
  ;[1 1 1] Does not check if exit index is valid
  (bind _output_get (Variables|/Game/OurStuff/Blueprints/Grid_Object_Parent.Grid_Object_Parent_C|Setindex Player (Variables|Default|GetexitIndex)))
  (Default|MovePlayer Player _output_get)
  (return))

(fn DPSIsExitingObjective
  (params (DPS :type Hide%20and%20Seek%20Player%20Object%20Reference))
  (Variables|/Game/OurStuff/Blueprints/Player/HideAndSeekPlayer.HideAndSeekPlayer_C|SetisMovementEnabled DPS true)
  (Variables|/Game/OurStuff/Blueprints/Player/HideAndSeekPlayer.HideAndSeekPlayer_C|SetisWithinAnObjective DPS false)
  (Variables|/Game/OurStuff/Blueprints/Player/HideAndSeekPlayer.HideAndSeekPlayer_C|SetobjectivePlayerIsIn DPS (Variables|Default|GetNULL_OBJECTIVE))
  (CallFunction|MovePlayerExitingObjective DPS))

(fn CheckifPlayerIsonAnEnterIndex
  (params (index :type Integer))
  (for _array_element (Variables|Default|GetentranceIndices)
    (if (== _array_element index)
      (return true)))
  (return false))
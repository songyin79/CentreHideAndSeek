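; Bug objective Blueprint for a hide-and-seek game, tracking whether the bug is captured through a flag on HideAndSeekGameState.
; BeginPlay runs the parent logic and resets BugIsCaptured to false, and UpdateGS sets it to true.
; SetObjectiveWidget creates a TimeCapsuleCaptured widget, despite the Bug name, and stores it as the objective widget.
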(event EventBeginPlay
  (|CallParentFunction)
  (bind _ashide_and_seek_game_state (Utilities|Casting|CastToHideAndSeekGameState (Game|GetGameState)))
  (Variables|/Game/OurStuff/HideAndSeekGameState.HideAndSeekGameState_C|SetbugIsCaptured _ashide_and_seek_game_state false))

(event EventSetObjectiveWidget
  (bind _returnvalue (UserInterface|CreateWidget "/Game/OurStuff/UI/TimeCapsuleCaptured.TimeCapsuleCaptured_C"))
  (Variables|Default|SetObjectiveWidget _returnvalue))

(event EventUpdateGS
  (bind _ashide_and_seek_game_state (Utilities|Casting|CastToHideAndSeekGameState (Game|GetGameState)))
  (Variables|/Game/OurStuff/HideAndSeekGameState.HideAndSeekGameState_C|SetbugIsCaptured _ashide_and_seek_game_state true))

(fn ConstructionScript
  (|CallParentFunction))
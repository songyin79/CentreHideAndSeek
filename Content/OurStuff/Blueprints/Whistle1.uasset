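; Whistle actor that clears minimap widgets and removes itself when notified that a DPS turn has passed.
; On that event it checks whether the local player pawn is a Student or DPS and picks the matching HUD from GameplayPC.
; It removes every widget in that minimap's Delete array, then destroys itself.
; If the pawn is neither type, the actor remains.
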(event EventBeginPlay)

(event Collision|EventActorBeginOverlap
  (params (OtherActor :type Actor%20Object%20Reference)))

(event EventTick
  (params (DeltaSeconds :type Float%20%28single-precision%29)))

(event EventNotifyDPSTurnPassed
  (bind _returnvalue (Game|GetPlayerController 0))
  (bind _returnvalue_2 (Pawn|GetControlledPawn _returnvalue))
  (bind _asgameplay_pc (Utilities|Casting|CastToGameplayPC _returnvalue))
  (Utilities|Casting|CastToStudent _returnvalue_2
    (:then
      (for _array_element (Variables|/Game/OurStuff/MiniMap/MiniMapWidget.MiniMapWidget_C|GetDelete (Variables|/Game/OurStuff/UI/HUD_Student.HUD_Student_C|GetMiniMapWidget (Variables|/Game/Blueprints/GamePlay/GameplayPC.GameplayPC_C|GetStudentHudRef _asgameplay_pc)))
        (Widget|RemovefromParent _array_element))
      (Actor|DestroyActor))
    (:CastFailed
      (Utilities|Casting|CastToDPS _returnvalue_2)
      (for _array_element_2 (Variables|/Game/OurStuff/MiniMap/MiniMapWidget.MiniMapWidget_C|GetDelete (Variables|/Game/OurStuff/UI/HUD_DPS.HUD_DPS_C|GetMiniMapWidget (Variables|/Game/Blueprints/GamePlay/GameplayPC.GameplayPC_C|GetDPSHudRef _asgameplay_pc)))
        (Widget|RemovefromParent _array_element_2))
      (Actor|DestroyActor))))

(fn ConstructionScript
  (|CallParentFunction))